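; BP_Player is a player Blueprint in the CapturesPlayer folder that steps through the level's TargetPoints.
; It gathers all TargetPoint actors on BeginPlay, and each Left key press moves it to the current target's transform without sweep.
; The target index increments after each successful move, with no wraparound or bounds check.
; The MoveAndCapture function is an empty stub, so no capture takes place here.
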(event EventBeginPlay
  (bind _outactors (Actor|GetAllActorsOfClass "/Script/Engine.TargetPoint"))
  (Variables|Default|SetTargets _outactors))

(event Input|KeyboardEvents|Left
  (params (Key :type Key%20Structure :default "None"))
  (:Pressed
    (bind _returnvalue (Transformation|SetActorTransform self (Transformation|GetActorTransform (Utilities|Array|Get(acopy) (Variables|Default|GetTargets) (Variables|Default|GetTargetsIndex)))))
    (if _returnvalue
      (Math|Integer|IncrementInt (Variables|Default|GetTargetsIndex)))))

(fn ConstructionScript)

(fn MoveandCapture)