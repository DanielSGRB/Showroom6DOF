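; BP_Button is a world-space interactable button made of a colored sphere and a text label, scaled from SphereSize at construction.
; Interact, Hovered and Unhovered fire event dispatchers and drive the sphere's "color" material parameter for hover feedback.
; With HoldState on, Interact toggles a selected state whose color overrides hover changes.
; Helper functions set or read selection and show or hide the button along with its collision.
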(event EventHovered
  (Default|CallOnButtonHovered self)
  (if (not (and (Variables|Default|GetholdState) (Variables|Default|GetisSelected)))
    (Rendering|Material|SetVectorParameterValueonMaterials (Variables|Default|GetSphere) "color" (Math|Conversions|ToVector(LinearColor) "(R=1.000000,G=0.997690,B=0.962442,A=1.000000)"))))

(event EventUnhovered
  (Default|CallOnButtonUnhovered self)
  (if (not (and (Variables|Default|GetholdState) (Variables|Default|GetisSelected)))
    (Rendering|Material|SetVectorParameterValueonMaterials (Variables|Default|GetSphere) "color" (Math|Conversions|ToVector(LinearColor)))))

(event EventInteract
  (params (interactionLocation :type Vector :default "0, 0, 0") (pawnInteractor :type BP%20SG%20Pawn%20Object%20Reference))
  (Default|CallOnButtonPressed self)
  (if (Variables|Default|GetholdState)
    (CallFunction|SetIsSelected (not (Variables|Default|GetisSelected)))))

(fn ConstructionScript
  (CallFunction|SetButtonAppearance (Variables|Default|Gettext)))

(fn SetButtonAppearance
  (params (text :type Text%20%28by%20ref%29))
  (Rendering|Components|TextRender|SetText (Variables|Default|GetTextRender) text)
  (Transformation|SetWorldScale3D (Variables|Default|GetSphere) (Math|Conversions|ToVector(Float) (/ (Variables|Default|GetsphereSize) 1e+02)))
  (Rendering|Components|TextRender|SetWorldSize (Variables|Default|GetTextRender) (/ (Math|Float|Max(Float) (Variables|Default|GetsphereSize) 35.0) 5.0))
  (Transformation|SetRelativeLocation (Variables|Default|GetTextRender) (Math|Vector|MakeVector 0.0 0.0 (/ (Variables|Default|GetsphereSize) 2.0)) false false))

(fn SetIsActive
  (params (isActive :type Boolean))
  (Rendering|SetActorHiddenInGame (not isActive))
  (Collision|SetActorEnableCollision isActive))

(fn SetIsSelected
  (params (isSelected :type Boolean))
  (bind _output_get (Variables|Default|SetisSelected isSelected))
  (Rendering|Material|SetVectorParameterValueonMaterials (Variables|Default|GetSphere) "color" (Math|Conversions|ToVector(LinearColor) (select _output_get "(R=0.000000,G=0.510601,B=0.661458,A=1.000000)" ""))))

(fn GetIsSelected
  (return (Variables|Default|GetisSelected)))