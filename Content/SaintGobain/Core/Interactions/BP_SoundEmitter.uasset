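; Interactable sound emitter that plays the audio matching the products currently selected in the map.
; WAVs are imported at runtime, and selection changes crossfade between two audio components at the tracked playback position.
; Invalid combinations switch other products to the closest valid set containing the last change, while all emitters inhibit updates.
; A spawned button toggles multicast playback, silences other emitters and blinks an area mesh on hover; a billboard shows sound state.
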(event OnAudioPlaybackPercent(Audio)
  (params (PlayingSoundWave :type Sound%20Wave%20Object%20Reference) (PlaybackPercent :type Float%20%28single-precision%29))
  ;[1 1 1] Percentage is actually count execution time, not absolute time. So if you execute Play with start time 3.0, percentage will start at 0 anyway.
  (Variables|Default|SetplaybackPercent PlaybackPercent))

(event OnAudioPlaybackPercent(Audio1)
  (params (PlayingSoundWave :type Sound%20Wave%20Object%20Reference) (PlaybackPercent :type Float%20%28single-precision%29))
  ;[1 1 1] Percentage is actually count execution time, not absolute time. So if you execute Play with start time 3.0, percentage will start at 0 anyway.
  (Variables|Default|SetplaybackPercent1 PlaybackPercent))

(event Custom|FetchAllSelectedProducts
  (params (lastProductSelected :type BP%20Product%20Object%20Reference))
  ;[1 1 1] Initialization
  ;;[1 1 1] Sound emitter has a mechanism to avoid falling into invalid product configurations. When a invalid product configuration is proposed, this flag is set to true until a valid configuration is found.
  (if (not (Variables|Default|GetshouldInhibitSoundUpdate))
    (Variables|Default|SetlastProductModified lastProductSelected)
    (Utilities|Array|Clear (Variables|Default|GetselectedProducts))
    (for _array_element (Variables|Default|GetallProductsInMap)
      (Utilities|Array|Add (Variables|Default|GetselectedProducts) (Default|GetSelectedProduct _array_element)))
    ;;[1 0.6403 0.5904] I'm sorry for this technical debt, future dev
    (if (Variables|Default|GetJustCalledUpdateAudioConfig)
      (Variables|Default|SetJustCalledUpdateAudioConfig false)
      (else
        (CallFunction|UpdateAudioConfiguration (Variables|Default|GetselectedProducts))
        (Variables|Default|SetJustCalledUpdateAudioConfig true)
        (Utilities|FlowControl|Delay 0.15)
        (Variables|Default|SetJustCalledUpdateAudioConfig false)))))

(event Custom|EditorInteract
  ;[1 0.1788 0] In Editor testing
  ;[0.2104 0.5208 1] BPI Interactable implementation
  (if (>= (CallFunction|FindIndexinListOfProductArrays (Variables|Default|GetselectedProducts)) 0)
    (if (Audio|Components|Audio|IsPlaying (Variables|Default|GetcurrentAudioComponent))
      (CallFunction|StopCurrentSound)
      (else
        (CallFunction|PlayCurrentSound)
        ;;[1 1 1] Stop other sounds by the button so the button has its state updated
        (for _array_element (Variables|Default|GetOtherSoundEmitters)
          (if (Default|GetIsSelected (CallFunction|GetButton _array_element))
            (Default|Interact (CallFunction|GetButton _array_element) "0, 0, 0")))
        (Utilities|FlowControl|Delay 5.0)
        (CallFunction|HideAudioArea)))
    (else
      (CallFunction|MulticastSetSoundIconState "NewEnumerator0"))))

(event Custom|MulticastSetSoundIconState
  (params (Index :type E_IconState%20Enum :default "NewEnumerator0"))
  ;[1 1 1] Play pause
  (CallFunction|SetSoundIconState Index))

(event Custom|StopBlinkingAudioArea
  ;[0.8472 1 0.04416] Audio area mesh opacity control
  (Utilities|FlowControl|Gate true) ; enters at Close
)

(event Custom|ImportAudiosFromFolder
  ;[1 1 1] Tried RuntimeAudio Importer, but receive this error when importing a wav from /saved folder :
  (Utilities|FlowControl|Delay 1.0)
  ;;[1 1 1] create runtime importer
  (bind _returnvalue (Class|RuntimeAudioImporterLibrary|CreateRuntimeAudioImporter))
  (CallFunction|TrytoImportAudiobyArrayIndex))

(event Custom|StartBlinkingAudioArea
  ;[0.8472 1 0.04416] Audio area mesh opacity control
  (if (not (Variables|Default|GetisShowingAudioArea))
    (Utilities|FlowControl|Sequence
      (:then_0
        (goto _label Open))
      (:then_1
        (Utilities|FlowControl|Gate true :!label _label
          (:Exit
            (Development|SetHiddeninGame (Variables|Default|GetmeshAudioArea) false false)
            (bind _opacity (Timeline|TL_BlinkingAudioArea PlayFromStart)
              (:Update
                (Rendering|Material|SetScalarParameterValueonMaterials (Variables|Default|GetmeshAudioArea) "opacityMult" _opacity))
              (:Finished
                (Development|SetHiddeninGame (Variables|Default|GetmeshAudioArea) true false)
                (goto _label)))))))))

(event Custom|ShowAudioArea
  (bind _tl_blinkingaudioarea (Variables|Default|GetTL_BlinkingAudioArea))
  (bind _tl_blinkingaudioarea_2 (Variables|Default|GetTL_BlinkingAudioArea))
  (bind _returnvalue (Components|Timeline|GetPlaybackPosition _tl_blinkingaudioarea))
  (bind _returnvalue_2 (- _returnvalue 0.5))
  ;[0.8472 1 0.04416] Audio area mesh opacity control
  (Variables|Default|SetisShowingAudioArea true)
  (Utilities|FlowControl|Sequence
    (:then_0
      (if (> _returnvalue_2 0.0)
        (Utilities|String|Reverse _tl_blinkingaudioarea_2)
        (else
          (Audio|Components|Audio|Play _tl_blinkingaudioarea_2))))
    (:then_1
      (Development|SetHiddeninGame (Variables|Default|GetmeshAudioArea) false false))
    (:then_2
      (Utilities|FlowControl|Delay (Math|Float|Absolute(Float) _returnvalue_2))
      (Audio|Components|Audio|Stop (Variables|Default|GetTL_BlinkingAudioArea)))))

(event Custom|HideAudioArea
  ;[0.8472 1 0.04416] Audio area mesh opacity control
  (Variables|Default|SetisShowingAudioArea false)
  (CallFunction|StopBlinkingAudioArea)
  (Utilities|String|Reverse (Variables|Default|GetTL_BlinkingAudioArea)))

(event Custom|StopCurrentSound
  ;[1 1 1] Play pause
  (Utilities|IsValid (Variables|Default|GetcurrentAudioComponent)
    (:Is%20Valid
      (Variables|Default|SetisPlayingAudio false)
      (CallFunction|MulticastStopSound (Variables|Default|GetcurrentAudioComponent))
      (CallFunction|MulticastSetSoundIconState "NewEnumerator1")
      (CallFunction|HideAudioArea))))

(event Custom|Delay
  (Utilities|FlowControl|Delay 0.2))

(event Custom|HandleButtonPressed
  (params (buttonRef :type BP%20Button%20Object%20Reference))
  ;[1 1 1] Initialization
  ;;[1 1 1] Interaction Button
  (CallFunction|Interact "0, 0, 0"))

(event Custom|HandleButtonHovered
  (params (buttonRef :type BP%20Button%20Object%20Reference))
  ;[1 1 1] Initialization
  ;;[1 1 1] Interaction Button
  (CallFunction|Hovered))

(event Custom|EditorTestProductList2
  ;[1 0.1788 0] In Editor testing
  (CallFunction|UpdateAudioConfiguration (.products (Utilities|Array|Get(acopy) (Variables|Default|GetproductToSoundArray) 2))))

(event Custom|HandleButtonUnhovered
  (params (buttonRef :type BP%20Button%20Object%20Reference))
  ;[1 1 1] Initialization
  ;;[1 1 1] Interaction Button
  (CallFunction|Unhovered))

(event Custom|HandleImportedSound
  (params (RuntimeAudioImporterObjectRef :type Runtime%20Audio%20Importer%20Library%20Object%20Reference) (SoundWaveRef :type Imported%20Sound%20Wave%20Object%20Reference) (Status :type ETranscodingStatus%20Enum%20%28by%20ref%29 :default "SuccessImporting"))
  (bind _producttosoundarray (Variables|Default|GetproductToSoundArray))
  ;[1 1 1] Tried RuntimeAudio Importer, but receive this error when importing a wav from /saved folder :
  ;;[1 1 1] handle sound import result
  (Utilities|FlowControl|Sequence
    (:then_0
      (if (Utilities|Enum|Equal(Enum) Status (Utilities|Enum|LiteralenumETranscodingStatus "SuccessImporting"))
        (Utilities|Array|SetArrayElem _producttosoundarray (stale Custom|TryToImportAudioByArrayIndex index) (Utilities|Struct|MakeS_ProductsArray (.products (Utilities|Array|Get(acopy) (Variables|Default|GetproductToSoundArray) (stale Custom|TryToImportAudioByArrayIndex index))) SoundWaveRef))
        (Development|PrintString (Utilities|String|Append "SUCCESS ON IMPORTING FILE " (Utilities|GetDisplayName SoundWaveRef) " of duration : " (Utilities|String|ToString(Float) (Variables|/Script/Engine.SoundBase|GetDuration (.soundwave (Utilities|Array|Get(acopy) _producttosoundarray (stale Custom|TryToImportAudioByArrayIndex index)))))))
        (else
          (Development|PrintString (Utilities|String|Append "Error on import: " (Utilities|String|EnumtoString Status))))))
    (:then_1
      (if (< (stale Custom|TryToImportAudioByArrayIndex index) (Utilities|Array|LastIndex (Variables|Default|GetproductToSoundArray)))
        (CallFunction|TrytoImportAudiobyArrayIndex (+ (stale Custom|TryToImportAudioByArrayIndex index) 1))
        (else
          (CallFunction|UpdateAudioConfiguration (Variables|Default|GetselectedProducts)))))))

(event Custom|TryToImportAudioByArrayIndex
  (params (index :type Integer))
  (bind _returnvalue (Class|KismetSystemLibrary|GetProjectSavedDirectory))
  (bind _returnvalue_2 (Game|GetPlatformName))
  (bind _producttosoundarray (Variables|Default|GetproductToSoundArray))
  (bind _audiofilesandroidpath (Variables|Default|GetAudioFilesAndroidPath))
  (bind _returnvalue_3 (Utilities|Enum|Equal(Enum) _returnvalue_2 "Windows"))
  (bind _output (Utilities|Array|Get(acopy) _producttosoundarray index))
  (bind _returnvalue_4 (Utilities|String|SelectString _returnvalue _audiofilesandroidpath _returnvalue_3))
  (bind _returnvalue_5 (Utilities|GetDisplayName (.soundwave _output)))
  (bind _returnvalue_6 (Utilities|String|Append _returnvalue_4 _returnvalue_5 ".wav"))
  ;[1 1 1] Tried RuntimeAudio Importer, but receive this error when importing a wav from /saved folder :
  (Development|PrintString (Utilities|String|Append "Requesting import of : " _returnvalue_6))
  (Class|RuntimeAudioImporterLibrary|ImportAudiofromFile (stale Custom|ImportAudiosFromFolder _returnvalue) _returnvalue_6 "Auto")
  (EventDispatchers|AssignOnResult (stale Custom|ImportAudiosFromFolder _returnvalue) (delegate Custom|HandleImportedSound)))

(event Custom|LoopCurrentAudioIfPossible
  ;[1 1 1] Play pause
  ;;[0.4358 0 1] Looping for imported Audio
  (CallFunction|ResetImportedAudioifReachedEnd))

(event Custom|MulticastStopSound
  (params (Target :type Audio%20Component%20Object%20Reference))
  ;[1 1 1] Play pause
  (Audio|Components|Audio|Stop Target)
  ;;[0.4358 0 1] Looping for imported Audio
  (Utilities|Time|PauseTimerbyHandle (stale Custom|MulticastPlaySound _returnvalue)))

(event Custom|InitializeEmissor
  ;[1 1 1] Initialization
  (for _array_element (Variables|Default|GetallProductsInMap)
    (EventDispatchers|BindEventtoOnProductSelected _array_element (EventDispatchers|CreateEvent :!event Custom|FetchAllSelectedProducts)))
  (CallFunction|FetchAllSelectedProducts))

(event Custom|EditorTestProductList0
  ;[1 0.1788 0] In Editor testing
  (CallFunction|UpdateAudioConfiguration (.products (Utilities|Array|Get(acopy) (Variables|Default|GetproductToSoundArray)))))

(event Custom|MulticastPlaySound
  (params (Target :type Audio%20Component%20Object%20Reference) (StartTime :type Float%20%28single-precision%29))
  ;[1 1 1] Play pause
  (bind _asimported_sound_wave (Utilities|Casting|CastToImportedSoundWave (Variables|/Script/Engine.AudioComponent|GetSound Target))
    (:then
      (Class|ImportedSoundWave|RewindPlaybackTime _asimported_sound_wave StartTime)
      (Audio|Components|Audio|Play Target 0.0))
    (:CastFailed
      (Audio|Components|Audio|Play Target StartTime)
      (Utilities|FlowControl|Sequence
        (:then_0
          ;;[0.4358 0 1] Looping for imported Audio
          (Utilities|FlowControl|DoOnce false
            (:Completed
              (bind _returnvalue (Utilities|Time|SetTimerbyEvent (delegate Custom|LoopCurrentAudioIfPossible) 0.1 true)))))
        (:then_1
          (Utilities|Time|UnpauseTimerbyHandle _returnvalue))))))

(event Custom|EditorTestProductList1
  ;[1 0.1788 0] In Editor testing
  (CallFunction|UpdateAudioConfiguration (.products (Utilities|Array|Get(acopy) (Variables|Default|GetproductToSoundArray) 1))))

(event Custom|PlayCurrentSound
  ;[1 1 1] Play pause
  (Utilities|IsValid (Variables|Default|GetcurrentAudioComponent)
    (:Is%20Valid
      (Variables|Default|SetisPlayingAudio true)
      (CallFunction|MulticastPlaySound (Variables|Default|GetcurrentAudioComponent) 0.0)
      (CallFunction|MulticastSetSoundIconState "NewEnumerator2")
      (CallFunction|ShowAudioArea))))

(event Custom|MulticastCrossFadeToNewAudioComponent
  (params (newSoundWave :type Sound%20Wave%20Object%20Reference) (nextAudioComp :type Audio%20Component%20Object%20Reference) (crossFadeDuration :type Float%20%28single-precision%29) (startTime :type Float%20%28single-precision%29))
  ;[1 1 1] Play pause
  (CallFunction|CrossFadetoNewAudioComponent newSoundWave nextAudioComp crossFadeDuration startTime))

(event EventHovered
  ;[0.2104 0.5208 1] BPI Interactable implementation
  (CallFunction|StartBlinkingAudioArea))

(event EventUnhovered
  ;[0.2104 0.5208 1] BPI Interactable implementation
  (CallFunction|StopBlinkingAudioArea))

(event EventEndPlay
  (params (EndPlayReason :type EEndPlayReason%20Enum :default "Destroyed"))
  (for _array_element (Variables|Default|GetproductToSoundArray)
    (bind _asimported_sound_wave (Utilities|Casting|CastToImportedSoundWave (.soundwave _array_element)))
    (Class|ImportedSoundWave|ReleaseMemory _asimported_sound_wave)))

(event EventInteract
  (params (interactionLocation :type Vector :default "0, 0, 0") (pawnInteractor :type BP%20SG%20Pawn%20Object%20Reference))
  ;[0.2104 0.5208 1] BPI Interactable implementation
  (if (>= (CallFunction|FindIndexinListOfProductArrays (Variables|Default|GetselectedProducts)) 0)
    (if (Audio|Components|Audio|IsPlaying (Variables|Default|GetcurrentAudioComponent))
      (CallFunction|StopCurrentSound)
      (else
        (CallFunction|PlayCurrentSound)
        ;;[1 1 1] Stop other sounds by the button so the button has its state updated
        (for _array_element (Variables|Default|GetOtherSoundEmitters)
          (if (Default|GetIsSelected (CallFunction|GetButton _array_element))
            (Default|Interact (CallFunction|GetButton _array_element) "0, 0, 0")))
        (Utilities|FlowControl|Delay 5.0)
        (CallFunction|HideAudioArea)))
    (else
      (CallFunction|MulticastSetSoundIconState "NewEnumerator0"))))

(event EventBeginPlay
  ;[1 1 1] Initialization
  (CallFunction|ImportAudiosfromFolder)
  (Utilities|FlowControl|Sequence
    (:then_0
      ;;[1 1 1] Interaction Button
      (bind _returnvalue (Game|SpawnActorfromClass "/Game/SaintGobain/Core/Interactions/BP_Button.BP_Button_C" (Transformation|GetActorTransform) "Undefined" 0 3e+01 "" true 0))
      (Default|SetIsActive _returnvalue false)
      (Default|SetButtonAppearance _returnvalue (Utilities|Text|FormatText "Sound {Number}" (Utilities|String|ToString(Integer) (Variables|Default|GetNumber))))
      (bind _output_get (Variables|Default|Setbutton _returnvalue))
      (Utilities|FlowControl|Sequence
        (:then_0
          (EventDispatchers|AssignOnButtonPressed _output_get (delegate Custom|HandleButtonPressed)))
        (:then_1
          (EventDispatchers|AssignOnButtonHovered _output_get (delegate Custom|HandleButtonHovered)))
        (:then_2
          (EventDispatchers|AssignOnButtonUnhovered _output_get (delegate Custom|HandleButtonUnhovered)))))
    (:then_1
      (if (Networking|IsServer)
        (CallFunction|InitializeEmissor)
        (Utilities|FlowControl|Delay 1.0) ; Making Sure every BP_SoundEmitter is spawned
        (bind _outactors (Actor|GetAllActorsOfClass "BP_SoundEmitter_C"))
        (bind _output_get_2 (Variables|Default|SetOtherSoundEmitters _outactors))
        (Utilities|Array|RemoveItem _output_get_2 self)))))

(fn ConstructionScript
  (bind _output_get (Variables|Default|SetcurrentAudioComponent (Variables|Default|GetAudio)))
  (Audio|Components|Audio|SetSound _output_get (.soundwave (Utilities|Array|Get(acopy) (Variables|Default|GetproductToSoundArray))))
  (Rendering|Material|SetVectorParameterValueonMaterials (Variables|Default|GetmeshAudioArea) "color" (Math|Conversions|ToVector(LinearColor) "(R=0.535028,G=1.000000,B=0.000000,A=1.000000)")))

(fn UpdateAudioConfiguration
  (params (selectedProducts :type Array%20of%20E_Products%20Enums :default "NewEnumerator21"))
  (bind _listindex (CallFunction|FindIndexinListOfProductArrays selectedProducts))
  (bind _audio (Variables|Default|GetAudio))
  (bind _currentaudiocomponent (Variables|Default|GetcurrentAudioComponent))
  (bind _sound (Variables|/Script/Engine.AudioComponent|GetSound _currentaudiocomponent))
  (bind _duration (Variables|/Script/Engine.SoundBase|GetDuration _sound))
  (Variables|Default|SetselectedProducts selectedProducts)
  (if (>= _listindex 0)
    ;[1 1 1] Percentage is actually count execution time, not absolute time. So if you execute Play with start time 3.0, percentage will start at 0 anyway. Because of that I saved and added lastStartTimeAssigned. The % is to wrap around time considering the file duration
    (Variables|Default|SetlastStartTimeAssigned (Math|Float|%(Float) (+ (Variables|Default|GetlastStartTimeAssigned) (* _duration (select (== (Variables|Default|GetcurrentAudioComponent) (Variables|Default|GetAudio1)) (Variables|Default|GetplaybackPercent1) (Variables|Default|GetplaybackPercent))) (* (Utilities|Time|GetWorldDeltaSeconds) 4.0)) _duration))
    (CallFunction|MulticastCrossFadetoNewAudioComponent (.soundwave (Utilities|Array|Get(acopy) (Variables|Default|GetproductToSoundArray) _listindex)) (select (== _audio (Variables|Default|GetcurrentAudioComponent)) (Variables|Default|GetAudio1) _audio) 0.5 (Variables|Default|GetlastStartTimeAssigned))
    (CallFunction|MulticastSetSoundIconState (select (Audio|Components|Audio|IsPlaying (Variables|Default|GetcurrentAudioComponent)) "NewEnumerator2" "NewEnumerator1"))
    (else
      (bind _outactors (Actor|GetAllActorsOfClass "BP_SoundEmitter_C"))
      ;[1 1 1] Making sure no sound emitter in the level will react to product changes while we are coming with a valid product list
      (for _array_element _outactors
        (CallFunction|SetShouldInhibitSoundUpdate _array_element true))
      (bind _avalidlist (CallFunction|FindValidProductListforRemainingProducts (Variables|Default|GetselectedProducts) (Variables|Default|GetlastProductModified)))
      (CallFunction|ChangeSelectiononRemainingProducts _avalidlist (Variables|Default|GetlastProductModified))
      (for _array_element_2 _outactors
        (CallFunction|SetShouldInhibitSoundUpdate _array_element_2 false)
        (CallFunction|FetchAllSelectedProducts _array_element_2 (Variables|Default|GetlastProductModified))))))

(fn FindIndexinListOfProductArrays
  (params (products :type Array%20of%20E_Products%20Enums :default "NewEnumerator21"))
  (for (_array_element _array_index) (Variables|Default|GetproductToSoundArray)
    (if (== (Utilities|Array|Length (.products _array_element)) (Utilities|Array|Length products))
      (LocalVariables|SettempProductConfiguration (.products _array_element))
      (LocalVariables|SetareArraysDifferent false)
      (for _array_element_2 products
        (if (>= (Utilities|Array|FindItem (LocalVariables|GettempProductConfiguration) _array_element_2) 0)
          (Utilities|Array|RemoveIndex (LocalVariables|GettempProductConfiguration) (Utilities|Array|FindItem (LocalVariables|GettempProductConfiguration) _array_element_2))
          (else
            (LocalVariables|SetareArraysDifferent true))))
      (if (not (LocalVariables|GetareArraysDifferent))
        (return _array_index))))
  (return -1))

(fn CrossFadetoNewAudioComponent
  (params (newSoundWave :type Sound%20Wave%20Object%20Reference) (nextAudioComp :type Audio%20Component%20Object%20Reference) (crossFadeDuration :type Float%20%28single-precision%29) (startTime :type Float%20%28single-precision%29))
  (LocalVariables|SetaudioStartTime startTime)
  (bind _output_get (LocalVariables|SetlNextComp nextAudioComp))
  (Audio|Components|Audio|SetSound _output_get newSoundWave)
  (Utilities|FlowControl|Sequence
    (:then_0
      (Development|PrintString (Utilities|String|Append "Start TIME   " (Utilities|String|ToString(Float) (LocalVariables|GetaudioStartTime))) true true "(R=0.981207,G=0.000000,B=1.000000,A=1.000000)" 1e+01)
      (bind _asimported_sound_wave (Utilities|Casting|CastToImportedSoundWave newSoundWave))
      (Class|ImportedSoundWave|RewindPlaybackTime _asimported_sound_wave (LocalVariables|GetaudioStartTime))
      (LocalVariables|SetaudioStartTime 0.0))
    (:then_1
      (if (Audio|Components|Audio|IsPlaying (Variables|Default|GetcurrentAudioComponent))
        (Audio|Components|Audio|FadeOut (Variables|Default|GetcurrentAudioComponent) crossFadeDuration 0.0 "Linear" :!class /Script/Engine.AudioComponent)
        (Audio|Components|Audio|FadeIn (LocalVariables|GetlNextComp) crossFadeDuration 1.0 (LocalVariables|GetaudioStartTime) "Linear" :!class /Script/Engine.AudioComponent)))
    (:then_2
      (Variables|Default|SetcurrentAudioComponent (LocalVariables|GetlNextComp)))))

(fn SetSoundIconState
  (params (Index :type E_IconState%20Enum :default "NewEnumerator0"))
  (Rendering|Components|Sprite|SetSprite (Variables|Default|GetBillboard) (Utilities|Select :Index Index :NewEnumerator0 "/Game/SaintGobain/Art/Interactions/T_SoundDisable_D.T_SoundDisable_D" :NewEnumerator1 "/Game/SaintGobain/Art/Interactions/T_SoundEnabledUnactive_D.T_SoundEnabledUnactive_D" :NewEnumerator2 "/Game/SaintGobain/Art/Interactions/T_SoundEnableActive_D.T_SoundEnableActive_D")))

(fn FindValidProductListforRemainingProducts
  (params (currentList :type Array%20of%20E_Products%20Enums :default "NewEnumerator21") (lastProductModified :type BP%20Product%20Object%20Reference))
  (bind _productselected (Default|GetSelectedProduct lastProductModified))
  ;[1 1 1] Valid list must contain last selected product
  (for _array_element (Variables|Default|GetproductToSoundArray)
    (LocalVariables|Settemp (.products (Utilities|Struct|BreakS_ProductsArray _array_element)))
    (if (> (Utilities|Array|FindItem (LocalVariables|Gettemp) _productselected) -1)
      (Utilities|Array|RemoveIndex (LocalVariables|Gettemp) (Utilities|Array|FindItem (LocalVariables|Gettemp) _productselected))
      (Utilities|Array|Add (LocalVariables|GetpossibleLists) (Utilities|Struct|MakeS_ProductsArray (LocalVariables|Gettemp)))))
  ;[1 1 1] Current (invalid) list without last selected product
  (bind _output_get (LocalVariables|Settemp currentList))
  (Utilities|Array|RemoveIndex _output_get (Utilities|Array|FindItem _output_get _productselected))
  (LocalVariables|SetbiggestIntersectionSize -1)
  ;[1 1 1] Find list with most elements in common with current (invalid) list
  (for _array_element_2 (LocalVariables|GetpossibleLists)
    (if (> (CallFunction|GetArraysIntersection (LocalVariables|Gettemp) (.products (Utilities|Struct|BreakS_ProductsArray _array_element_2))) (LocalVariables|GetbiggestIntersectionSize))
      (LocalVariables|SetvalidList (.products (Utilities|Struct|BreakS_ProductsArray _array_element_2)))
      (LocalVariables|SetbiggestIntersectionSize (CallFunction|GetArraysIntersection (LocalVariables|Gettemp) (.products (Utilities|Struct|BreakS_ProductsArray _array_element_2))))))
  (return (LocalVariables|GetvalidList)))

(fn ChangeSelectiononRemainingProducts
  (params (validList :type Array%20of%20E_Products%20Enums :default "NewEnumerator21") (lastModifiedProduct :type BP%20Product%20Object%20Reference))
  (LocalVariables|SetlValidList validList)
  (Utilities|FlowControl|Sequence
    (:then_0
      (for _array_element (Variables|Default|GetallProductsInMap)
        (if (!= _array_element lastModifiedProduct)
          (Utilities|Array|Add (LocalVariables|GetremainingProducts) _array_element))))
    (:then_1
      (for _array_element_2 (LocalVariables|GetremainingProducts)
        (bind _keys (Utilities|Map|Keys (Variables|/Game/SaintGobain/Core/Interactions/BP_Product.BP_Product_C|GetproductToMaterials _array_element_2)))
        (bind _array_element_3 (Utilities|Array|ForEachLoopwithBreak _keys :!label _label)
          (:LoopBody
            (if (> (Utilities|Array|FindItem (LocalVariables|GetlValidList) _array_element_3) -1)
              (Default|SelectProductasifInteractingwithMenu _array_element_2 _array_element_3)
              (Utilities|Array|RemoveIndex (LocalVariables|GetlValidList) (Utilities|Array|FindItem (LocalVariables|GetlValidList) _array_element_3))
              (goto _label Break))))))))

(fn GetArraysIntersection
  (params (A :type Array%20of%20E_Products%20Enums :default "NewEnumerator21") (B :type Array%20of%20E_Products%20Enums :default "NewEnumerator21"))
  (bind _output_get (LocalVariables|SetlA A))
  (bind _output_get_2 (LocalVariables|SetlB B))
  (for _array_element _output_get
    (if (> (Utilities|Array|FindItem _output_get_2 _array_element) -1)
      (Utilities|Array|RemoveIndex _output_get_2 (Utilities|Array|FindItem _output_get_2 _array_element))
      (Math|Integer|IncrementInt (LocalVariables|GetintersectionSize))))
  (return (LocalVariables|GetintersectionSize)))

(fn SetShouldInhibitSoundUpdate
  (params (shouldInhibitSoundUpdate :type Boolean))
  (Variables|Default|SetshouldInhibitSoundUpdate shouldInhibitSoundUpdate))

(fn GetShouldInhibitSoundUpdate
  (return (Variables|Default|GetshouldInhibitSoundUpdate)))

(fn GetButton
  (return (Variables|Default|Getbutton)))

(fn FindIndexbyStringinSoundArray
  (params (fileName :type String) (productToSoundArray :type Array%20of%20S%20Products%20Array%20Structures))
  (bind (_lefts _rights _returnvalue) (Utilities|String|Split fileName ""))
  (for (_array_element _array_index) productToSoundArray
    (if (Utilities|Enum|Equal(Enum) (Utilities|GetDisplayName (.soundwave (Utilities|Struct|BreakS_ProductsArray _array_element))) (Utilities|String|SelectString _lefts fileName _returnvalue))
      (return _array_index)))
  (return -1))

(fn ResetImportedAudioifReachedEnd
  (bind _asimported_sound_wave (Utilities|Casting|CastToImportedSoundWave (Variables|/Script/Engine.AudioComponent|GetSound (Variables|Default|GetcurrentAudioComponent))))
  (bind _returnvalue (Class|ImportedSoundWave|GetPlaybackPercentage _asimported_sound_wave))
  (if (== _returnvalue 1e+02)
    (Class|ImportedSoundWave|RewindPlaybackTime _asimported_sound_wave 0.0)))