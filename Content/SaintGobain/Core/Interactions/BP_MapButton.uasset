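; BP_MapButton is an interactable sphere button that travels to a chosen map, ends the visit or restarts the room.
; Interact calls the game instance's ChangeMap, except when Map is InitialMap, where the button type either toggles a confirmation menu for returning there or resets all products.
; The construction script sets a dynamic material with the map's cubemap or a color, plus a label, both scaled by SphereSize.
; SetIsActive toggles visibility and collision.
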(event Custom|SetIsActive
  (params (isActive :type Boolean))
  (bind _returnvalue (not isActive))
  (Collision|SetActorEnableCollision isActive)
  (Rendering|SetActorHiddenInGame _returnvalue)
  (if (and _returnvalue (Utilities|IsValid (Variables|Default|GetconfirmationMenu)))
    (Actor|DestroyActor (Variables|Default|GetconfirmationMenu))))

(event Custom|HandleConfirmationResult
  (params (isResultYes :type Boolean))
  (if isResultYes
    (bind _asbp_sggame_instance (Utilities|Casting|CastToBP_SGGameInstance (Game|GetGameInstance)))
    (Default|ChangeMap _asbp_sggame_instance "NewEnumerator5")
    (else
      (Actor|DestroyActor (Variables|Default|GetconfirmationMenu)))))

(event EventInteract
  (params (interactionLocation :type Vector :default "0, 0, 0") (pawnInteractor :type BP%20SG%20Pawn%20Object%20Reference))
  (if (Utilities|Enum|Equal(Enum) (Variables|Default|Getmap) "NewEnumerator5")
    (switch int (Variables|Default|GetNotMapButtonType)
      (:0
        (Utilities|IsValid (Variables|Default|GetconfirmationMenu)
          (:Is%20Valid
            (Actor|DestroyActor (Variables|Default|GetconfirmationMenu)))
          (:Is%20Not%20Valid
            (bind _returnvalue (Game|SpawnActorfromClass "/Game/SaintGobain/Core/Menus/BP_ConfirmationMenu.BP_ConfirmationMenu_C" (Math|Transform|ComposeTransforms (Transformation|GetActorTransform) (Math|Transform|MakeTransform "0, 0,30.000000" "0, 0, 0" "1,1,1")) "Undefined" 0 0))
            (bind _output_get (Variables|Default|SetconfirmationMenu _returnvalue))
            (EventDispatchers|BindEventtoOnConfirmationResult _output_get (delegate Custom|HandleConfirmationResult)))))
      (:1
        (bind _outactors (Actor|GetAllActorsOfClass "/Game/SaintGobain/Core/Interactions/BP_Product.BP_Product_C"))
        (for _array_element _outactors
          (Default|ResetProduct _array_element))
        (Default|CallOnProductSelected (Utilities|Array|Get(acopy) _outactors) (Utilities|Array|Get(acopy) _outactors))))
    (else
      (bind _asbp_sggame_instance (Utilities|Casting|CastToBP_SGGameInstance (Game|GetGameInstance)))
      (Default|ChangeMap _asbp_sggame_instance (Variables|Default|Getmap)))))

(fn ConstructionScript
  (bind _returnvalue (Rendering|Material|CreateDynamicMaterialInstance (Variables|Default|GetSphere) 0 "/Game/SaintGobain/Art/Interactions/M_Maps.M_Maps" "None" :!class /Script/Engine.PrimitiveComponent))
  (Variables|Default|SetsphereMaterial _returnvalue)
  (CallFunction|SetButtonAppearance (Variables|Default|Getmap)))

(fn SetButtonAppearance
  (params (map :type E_Maps%20Enum :default "NewEnumerator5"))
  (Rendering|Material|SetTextureParameterValue (Variables|Default|GetsphereMaterial) "texture" (Utilities|Select :Index (Variables|Default|GetNotMapButtonType) :Option%200 "/Game/SaintGobain/Art/Interactions/Red.Red" :Option%201 "/Game/SaintGobain/Art/Interactions/Yellow.Yellow" :Option%202 (Utilities|Select :Index map :NewEnumerator5 "/Game/SaintGobain/Art/Interactions/Red.Red" :NewEnumerator0 "/Game/SaintGobain/Art/Interactions/T_HospitalReceptionCubemap_D.T_HospitalReceptionCubemap_D" :NewEnumerator1 "/Game/SaintGobain/Art/Interactions/T_HospitalCorridorCubemap_D.T_HospitalCorridorCubemap_D" :NewEnumerator2 "/Game/SaintGobain/Art/Interactions/T_HospitalRoomCubemap_D.T_HospitalRoomCubemap_D" :NewEnumerator3 "/Game/SaintGobain/Art/Interactions/T_HospitalOutpatientWardCubemap_D.T_HospitalOutpatientWardCubemap_D" :NewEnumerator4 "/Game/SaintGobain/Art/Interactions/T_ConferenceRoomCubemap_D.T_ConferenceRoomCubemap_D")))
  (Rendering|Components|TextRender|SetText (Variables|Default|GetTextRender) (Utilities|Select :Index (Variables|Default|GetNotMapButtonType) :Option%200 (Utilities|Text|MakeLiteralText "Encerrar 
Visita") :Option%201 (Utilities|Text|MakeLiteralText "Reiniciar 
Sala") :Option%202 (CallFunction|GetMapDisplayName map)))
  (Transformation|SetWorldScale3D (Variables|Default|GetSphere) (Math|Conversions|ToVector(Float) (/ (Variables|Default|GetsphereSize) 1e+02)))
  (Rendering|Components|TextRender|SetWorldSize (Variables|Default|GetTextRender) (/ (Math|Float|Max(Float) (Variables|Default|GetsphereSize) 35.0) 8.0))
  (Transformation|SetRelativeLocation (Variables|Default|GetTextRender) (Math|Vector|MakeVector 0.0 0.0 (/ (Variables|Default|GetsphereSize) 1.8)) false false))