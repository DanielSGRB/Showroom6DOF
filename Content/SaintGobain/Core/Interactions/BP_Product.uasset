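; BP_Product is an interactable product selector that swaps materials on linked static mesh actors to show the chosen product.
; Interacting from beyond a minimum distance opens a camera-facing menu between pawn and hit point, closing other products' menus.
; Menu choices pass through a multicast event to update name, logo and materials, cycling material sets across actors or hiding them when none exist.
; Reset restores the first product without firing the selection dispatcher.
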(event Custom|HandleNewProductSelected
  (params (selectedProduct :type E_Products%20Enum :default "NewEnumerator21"))
  (CallFunction|MulticastChangeProduct selectedProduct))

(event Custom|MulticastChangeProduct
  (params (productSelected :type E_Products%20Enum :default "NewEnumerator21"))
  (CallFunction|SetSelectedProduct productSelected false))

(event Custom|ActivateWidget
  (bind _widget (Variables|Default|GetWidget))
  ;[1 1 1] Widget Visibility
  (Development|SetHiddeninGame _widget false false)
  (Collision|SetCollisionProfileName _widget "UI" true :!class /Script/Engine.PrimitiveComponent)
  (for _array_element (Variables|Default|GetotherProducts)
    (CallFunction|DeactivateWidget _array_element)))

(event Custom|DeactivateWidget
  (bind _widget (Variables|Default|GetWidget))
  ;[1 1 1] Widget Visibility
  (Development|SetHiddeninGame _widget true false)
  (Collision|SetCollisionProfileName _widget "NoCollision" true :!class /Script/Engine.PrimitiveComponent))

(event Custom|SelectProductAsIfInteractingWithMenu
  (params (selectedProduct :type E_Products%20Enum :default "NewEnumerator21"))
  (Default|HandleProductButtonPressed (Variables|Default|GetButtonsMenu) selectedProduct true))

(event Custom|ResetProduct
  (bind _buttonsmenu (Variables|Default|GetButtonsMenu))
  (bind _keys (Utilities|Map|Keys (Variables|Default|GetproductToMaterials)))
  (CallFunction|SetSelectedProduct (Utilities|Array|Get(acopy) _keys) true)
  (bind _output_get (Variables|/Game/SaintGobain/Core/Menus/W_ProductsMenu.W_ProductsMenu_C|Setselected _buttonsmenu (Utilities|Array|Get(acopy) _keys)))
  (Default|SetOnlyOneButtonSelected _buttonsmenu _output_get))

(event EventBeginPlay
  (Utilities|FlowControl|Sequence
    (:then_0
      (CallFunction|DeactivateWidget)
      (bind _asw_product_logo (Utilities|Casting|CastToW_ProductLogo (UserInterface|GetUserWidgetObject (Variables|Default|GetProductLogoWidget))))
      (bind _output_get (Variables|Default|SetProductLogo _asw_product_logo))
      (Default|UpdateProductLogo _output_get (Variables|Default|GetproductSelected))
      (CallFunction|SetSelectedProduct (Variables|Default|GetproductSelected) false)
      (bind _asw_products_menu (Utilities|Casting|CastToW_ProductsMenu (UserInterface|GetUserWidgetObject (Variables|Default|GetWidget))))
      (bind _output_get_2 (Variables|Default|SetButtonsMenu _asw_products_menu))
      (bind _keys (Utilities|Map|Keys (Variables|Default|GetproductToMaterials)))
      (Default|GenerateProductListButtons _output_get_2 _keys (Variables|Default|GetproductSelected))
      (EventDispatchers|BindEventtoOnProductSelectedWidget _output_get_2 (delegate Custom|HandleNewProductSelected))
      (EventDispatchers|AssignOnClosePressed _output_get_2 (EventDispatchers|CreateEvent :!event Custom|DeactivateWidget)))
    (:then_1
      (Utilities|FlowControl|Delay 1.0) ; Making Sure every BP_Product is spawned
      (bind _outactors (Actor|GetAllActorsOfClass "BP_Product_C"))
      (bind _output_get_3 (Variables|Default|SetotherProducts _outactors))
      (Utilities|Array|RemoveItem _output_get_3 self))))

(event EventInteract
  (params (interactionLocation :type Vector :default "0, 0, 0") (pawnInteractor :type BP%20SG%20Pawn%20Object%20Reference))
  (bind _camera (Variables|/Game/SaintGobain/Core/Player/BP_SGPawn.BP_SGPawn_C|GetCamera pawnInteractor))
  (bind _returnvalue (Transformation|GetWorldLocation _camera))
  (bind _returnvalue_2 (Math|Vector|Lerp(Vector) interactionLocation _returnvalue 0.6))
  ;[1 1 1] Pop widget
  (if (> (Math|Vector|Distance(Vector) interactionLocation _returnvalue) (Math|Float|MakeLiteralFloat 2e+02))
    (Transformation|SetWorldLocationAndRotation (Variables|Default|GetWidget) _returnvalue_2 (Math|Rotator|FindLookatRotation _returnvalue_2 _returnvalue) false true)
    (CallFunction|ActivateWidget)))

(fn ConstructionScript)

(fn SetSelectedProduct
  (params (productSelected :type E_Products%20Enum :default "NewEnumerator21") (Reseting :type Boolean))
  (bind _output_get (Variables|Default|SetproductSelected productSelected))
  (Rendering|Components|TextRender|SetText (Variables|Default|GettextProductName) (CallFunction|GetProductName _output_get))
  (if Reseting
    _
    (else
      (Default|CallOnProductSelected self)))
  (Default|UpdateProductLogo (Variables|Default|GetProductLogo) _output_get)
  (if (.ReturnValue (Utilities|Map|Find (Variables|Default|GetproductToMaterials) _output_get))
    (for (_array_element _array_index) (Variables|Default|GetaffectedSMActors)
      (if (> (Utilities|Array|Length (.materials (.Value (Utilities|Map|Find (Variables|Default|GetproductToMaterials) _output_get)))) 0)
        (Rendering|SetActorHiddenInGame _array_element false)
        (Rendering|SetVisibility (Variables|/Script/Engine.StaticMeshActor|GetStaticMeshComponent _array_element) true true)
        (for (_array_element_2 _array_index_2) (.materialarray (Utilities|Array|Get(acopy) (.materials (.Value (Utilities|Map|Find (Variables|Default|GetproductToMaterials) _output_get))) (Math|Integer|%(Integer) _array_index (Utilities|Array|Length (.materials (.Value (Utilities|Map|Find (Variables|Default|GetproductToMaterials) _output_get)))))))
          (Rendering|Material|SetMaterial (Variables|/Script/Engine.StaticMeshActor|GetStaticMeshComponent _array_element) _array_index_2 _array_element_2))
        (else
          (Rendering|SetActorHiddenInGame _array_element true)
          (Rendering|SetVisibility (Variables|/Script/Engine.StaticMeshActor|GetStaticMeshComponent _array_element) false true))))
    (else
      (for _array_element_3 (Variables|Default|GetaffectedSMActors)
        (Rendering|SetActorHiddenInGame _array_element_3 true)
        (Rendering|SetVisibility (Variables|/Script/Engine.StaticMeshActor|GetStaticMeshComponent _array_element_3) false true)))))

(fn GetSelectedProduct
  (return (Variables|Default|GetproductSelected)))