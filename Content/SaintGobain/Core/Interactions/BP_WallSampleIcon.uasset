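; BP_WallSampleIcon is an interactable billboard icon, shown only on the server, that toggles wall cross-section samples in players' hands.
; Product selection sets its unavailable, inactive or active state and sprite via a product-to-mesh map.
; Interacting spawns or destroys mesh components on every BP_SGPawn's right-hand socket, and product changes update or remove them.
; Two wallcut meshes are localized by swapping to English materials instead of using the localization tool.
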(event Custom|HandleProductChange
  (params (productRef :type BP%20Product%20Object%20Reference))
  (bind _product (Variables|Default|Getproduct))
  (bind _producttowallsamplemeshmap (Variables|Default|GetproductToWallSampleMeshMap))
  (bind _productselected (Default|GetSelectedProduct _product))
  (bind (_value _returnvalue) (Utilities|Map|Find _producttowallsamplemeshmap _productselected))
  (if _returnvalue
    (CallFunction|SetState (Utilities|Select :Index (Variables|Default|Getstate) :NewEnumerator0 "NewEnumerator1" :NewEnumerator1 "NewEnumerator1" :NewEnumerator2 "NewEnumerator2"))
    (if (Utilities|Enum|Equal(Enum) (Variables|Default|Getstate) "NewEnumerator2")
      (CallFunction|MulticastUpdateSample _value))
    (else
      (CallFunction|SetState "NewEnumerator0")
      (CallFunction|DestroySamples))))

(event Custom|DestroySamples
  (for _array_element (Variables|Default|GetsamplesMeshComponents)
    (Components|DestroyComponent _array_element))
  (Utilities|Array|Clear (Variables|Default|GetsamplesMeshComponents)))

(event Custom|SpawnSamples
  (CallFunction|DestroySamples)
  (Utilities|FlowControl|Sequence
    (:then_0
      (bind _outactors (Actor|GetAllActorsOfClass "/Game/SaintGobain/Core/Player/BP_SGPawn.BP_SGPawn_C"))
      (Utilities|Array|Clear (Variables|Default|Getpawns))
      (for _array_element _outactors
        (Utilities|Array|Add (Variables|Default|Getpawns) _array_element)))
    (:then_1
      (for _array_element_2 (Variables|Default|Getpawns)
        (bind _returnvalue (AddComponent|AddStaticMeshComponent true))
        (Utilities|Array|Add (Variables|Default|GetsamplesMeshComponents) _returnvalue)
        (Transformation|AttachComponentToComponent _returnvalue (Variables|/Script/Engine.Actor|GetRootComponent (Variables|/Game/SaintGobain/Core/Player/BP_SGPawn.BP_SGPawn_C|GethandRight _array_element_2)) "socketWallcut" "SnapToTarget" "SnapToTarget" "KeepWorld" true)
        (CallFunction|UpdateSample _returnvalue (.Value (Utilities|Map|Find (Variables|Default|GetproductToWallSampleMeshMap) (Default|GetSelectedProduct (Variables|Default|Getproduct)))))))))

(event Custom|UpdateSample
  (params (smComponent :type Static%20Mesh%20Component%20Object%20Reference) (NewMesh :type Static%20Mesh%20Object%20Reference))
  (bind _returnvalue (Class|KismetInternationalizationLibrary|GetCurrentLanguage))
  (bind _returnvalue_2 (Utilities|Enum|Equal(Enum) _returnvalue "en"))
  ;[1 1 1] Since we only need to change language in 2 wallcuts and we already had the material in both languages, this will do for localization. If it gets more complex, its better to add text to the meshes in a blueprint and work with the localization tool.
  (Components|StaticMesh|SetStaticMesh smComponent NewMesh)
  (if (== NewMesh "/Game/SaintGobain/Art/Environment/WallCut/SM_WallCut00.SM_WallCut00")
    (Rendering|Material|SetMaterial smComponent 0 (select _returnvalue_2 "/Game/SaintGobain/Art/Environment/WallCut/M_WallCut00ENG.M_WallCut00ENG" "/Game/SaintGobain/Art/Environment/WallCut/M_WallCut00.M_WallCut00"))
    (elif (== NewMesh "/Game/SaintGobain/Art/Environment/WallCut/SM_WallCut05.SM_WallCut05")
      (Rendering|Material|SetMaterial smComponent 0 (select _returnvalue_2 "/Game/SaintGobain/Art/Environment/WallCut/M_WallCut05ENG.M_WallCut05ENG" "/Game/SaintGobain/Art/Environment/WallCut/M_WallCut05.M_WallCut05")))))

(event Custom|MulticastUpdateSample
  (params (NewMesh :type Static%20Mesh%20Object%20Reference))
  (for _array_element (Variables|Default|GetsamplesMeshComponents)
    (CallFunction|UpdateSample _array_element NewMesh)))

(event EventBeginPlay
  (if (Networking|IsServer)
    (Utilities|FlowControl|Sequence
      (:then_0
        (Utilities|IsValid (Variables|Default|Getproduct)
          (:Is%20Valid
            (EventDispatchers|AssignOnProductSelected (Variables|Default|Getproduct) (delegate Custom|HandleProductChange)))))
      (:then_1
        (CallFunction|HandleProductChange)))
    (else
      (Development|SetHiddeninGame (Variables|Default|GetBillboard) true false))))

(event EventInteract
  (params (interactionLocation :type Vector :default "0, 0, 0") (pawnInteractor :type BP%20SG%20Pawn%20Object%20Reference))
  (switch Utilities|FlowControl|Switch|SwitchonE_IconState (Variables|Default|Getstate)
    (:NewEnumerator1
      (CallFunction|SetState "NewEnumerator2")
      (CallFunction|SpawnSamples))
    (:NewEnumerator2
      (CallFunction|SetState "NewEnumerator1")
      (CallFunction|DestroySamples))))

(fn ConstructionScript)

(fn SetState
  (params (state :type E_IconState%20Enum :default "NewEnumerator0"))
  (bind _output_get (Variables|Default|Setstate state))
  (Rendering|Components|Sprite|SetSprite (Variables|Default|GetBillboard) (Utilities|Select :Index _output_get :NewEnumerator0 "/Game/SaintGobain/Art/Interactions/T_InfDisable_D.T_InfDisable_D" :NewEnumerator1 "/Game/SaintGobain/Art/Interactions/T_InfEnabledUnactive_D.T_InfEnabledUnactive_D" :NewEnumerator2 "/Game/SaintGobain/Art/Interactions/T_InfEnabledActive_D.T_InfEnabledActive_D")))

(fn GetState
  (return (Variables|Default|Getstate)))