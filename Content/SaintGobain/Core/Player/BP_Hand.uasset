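; VR hand actor providing mirrored mesh, avatar color and a laser pointer for widgets, interactables and teleporting.
; While the hand is active, a looping timer line-traces to update laser and hover, with multicasts for active state and color.
; Trigger presses widgets, messages BPI_Interactable actors, or otherwise starts teleport aiming, executed on release via BP_SGPawn.
; Teleport draws an animated HISM parabola, valid only when all four guardian-area corners project onto the navmesh.
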(event Custom|BeginTeleportTick
  ;[0.4209 0.1419 1] Teleport
  (Default|CallOnTeleportStarted)
  (Development|SetHiddeninGame (Variables|Default|GethismTeleportPath) false false)
  (Rendering|SetVisibility (Variables|Default|GetmeshLaserPoint) false false)
  (bind _returnvalue (Utilities|Time|SetTimerbyEvent (delegate Custom|TeleportTick) 0.01 true)))

(event Custom|TryToExecuteTeleport
  (bind _teleporthitresult (Variables|Default|GetteleportHitResult))
  (bind (_projectedcenter _isvalidplace) (CallFunction|ProjectPlayAreatoNavigationSystem (.impactpoint _teleporthitresult)))
  ;[0.4209 0.1419 1] Teleport
  (CallFunction|EndTeleportTick)
  (bind _asbp_sgpawn (Utilities|Casting|CastToBP_SGPawn (Components|GetOwner))
    (:then
      (if (and (.bblockinghit _teleporthitresult) _isvalidplace)
        (Default|TeleporttoLocation _asbp_sgpawn _projectedcenter)))
    (:CastFailed
      _))
  (Variables|Default|SetisTeleporting false))

(event Custom|MulticastSetLaserColor
  (params (traceHitResult :type E_TraceHitResult%20Enum :default "NewEnumerator0"))
  (CallFunction|SetLaserColor traceHitResult))

(event Custom|PressTriggerAction
  (bind _interacthitresult (Variables|Default|GetinteractHitResult))
  (if (Variables|Default|GetisActive)
    (Utilities|Casting|CastToWidgetComponent (.hitcomponent _interacthitresult)
      (:then
        (Class|WidgetInteractionComponent|SetCustomHitResult (Variables|Default|GetWidgetInteraction) (Variables|Default|GetinteractHitResult))
        (Class|WidgetInteractionComponent|PressPointerKey (Variables|Default|GetWidgetInteraction) "LeftMouseButton"))
      (:CastFailed
        (if (Utilities|DoesObjectImplementInterface (.hitactor _interacthitresult) "/Game/SaintGobain/Core/Interactions/BPI_Interactable.BPI_Interactable_C")
          (bind _asbp_sgpawn (Utilities|Casting|CastToBP_SGPawn (Components|GetOwner)))
          (Class|BPIInteractable|Interact(Message) (.hitactor _interacthitresult) (.impactpoint _interacthitresult) _asbp_sgpawn)
          (else
            (Variables|Default|SetisTeleporting true)
            (CallFunction|BeginTeleportTick)))))))

(event Custom|TeleportTick
  (bind _widgetinteraction (Variables|Default|GetWidgetInteraction))
  ;[0.4209 0.1419 1] Teleport
  (bind (_outhit _parabolapath) (CallFunction|ParabolaTrace (Transformation|GetWorldLocation _widgetinteraction) (* (Math|Vector|GetForwardVector _widgetinteraction) 8e+02) "0, 0,-980.000000" 0.03 60 (Utilities|Array|MakeArray "ObjectTypeQuery1")))
  (bind _output_get (Variables|Default|SetteleportHitResult _outhit))
  (CallFunction|DrawTeleportGizmo _parabolapath (.projectedCenter (CallFunction|ProjectPlayAreatoNavigationSystem (.Location (Collision|BreakHitResult _output_get)))) (and (.bBlockingHit (Collision|BreakHitResult _output_get)) (.IsValidPlace (CallFunction|ProjectPlayAreatoNavigationSystem (.Location (Collision|BreakHitResult _output_get)))))))

(event Custom|ReleaseTriggerAction
  (Class|WidgetInteractionComponent|ReleasePointerKey (Variables|Default|GetWidgetInteraction) "LeftMouseButton")
  (if (Variables|Default|GetisTeleporting)
    (CallFunction|TrytoExecuteTeleport)))

(event Custom|EndTeleportTick
  ;[0.4209 0.1419 1] Teleport
  (Default|CallOnTeleportEnded)
  (Development|SetHiddeninGame (Variables|Default|GethismTeleportPath) true false)
  (Rendering|SetVisibility (Variables|Default|GetmeshLaserPoint) true false)
  (Utilities|Time|ClearandInvalidateTimerbyHandle (stale Custom|BeginTeleportTick _returnvalue)))

(event Custom|TraceTick
  (bind _returnvalue (Math|Float|MakeLiteralFloat 1e+04))
  (bind _widgetinteraction (Variables|Default|GetWidgetInteraction))
  (bind _returnvalue_2 (Transformation|GetWorldLocation _widgetinteraction))
  (bind _returnvalue_3 (Math|Vector|GetForwardVector _widgetinteraction))
  (bind _returnvalue_4 (* _returnvalue_3 _returnvalue))
  (bind _returnvalue_5 (+ _returnvalue_2 _returnvalue_4))
  ;[1 1 1] Widget and interactable trace
  (if (not (Variables|Default|GetisTeleporting))
    (bind (_outhit _returnvalue_6) (CallFunction|Trace _returnvalue))
    (if _returnvalue_6
      (bind _output_get (Variables|Default|SetinteractHitResult _outhit))
      (CallFunction|ScaleMeshBetweenPoints (Variables|Default|GetmeshLaserPath) (Transformation|GetWorldLocation (Variables|Default|GetWidgetInteraction)) (.ImpactPoint (Collision|BreakHitResult _output_get)))
      (Transformation|SetWorldLocation (Variables|Default|GetmeshLaserPoint) (.ImpactPoint (Collision|BreakHitResult _output_get)) false true)
      (CallFunction|MulticastSetLaserColor (select (Utilities|DoesObjectImplementInterface (.HitActor (Collision|BreakHitResult _output_get)) "/Game/SaintGobain/Core/Interactions/BPI_Interactable.BPI_Interactable_C") "NewEnumerator2" "NewEnumerator1"))
      (if (!= (Variables|Default|GetlastHoveredInteractable) (.HitActor (Collision|BreakHitResult _output_get)))
        (Utilities|FlowControl|Sequence
          (:then_0
            (Utilities|IsValid (Variables|Default|GetlastHoveredInteractable)
              (:Is%20Valid
                (Class|BPIInteractable|Unhovered(Message) (Variables|Default|GetlastHoveredInteractable)))))
          (:then_1
            (bind _output_get_2 (Variables|Default|SetlastHoveredInteractable (.HitActor (Collision|BreakHitResult _output_get))))
            (Class|BPIInteractable|Hovered(Message) _output_get_2))))
      (else
        (CallFunction|ScaleMeshBetweenPoints (Variables|Default|GetmeshLaserPath) _returnvalue_2 _returnvalue_5)
        (Transformation|SetWorldLocation (Variables|Default|GetmeshLaserPoint) _returnvalue_5 false true)
        (CallFunction|SetLaserColor "NewEnumerator0")))))

(event Custom|MulticastSetHandActive
  (params (isActive :type Boolean))
  (if (Variables|Default|GetisShowingLaser)
    (Development|SetHiddeninGame (Variables|Default|GetmeshLaserPoint) (not isActive) false)
    (Variables|/Script/UMG.WidgetInteractionComponent|SetbEnableHitTesting (Variables|Default|GetWidgetInteraction) isActive)
    (bind _output_get (Variables|Default|SetisActive isActive))
    (if _output_get
      (CallFunction|StartTraceTick)
      (else
        (CallFunction|StopTraceTick)))))

(event Custom|StartTraceTick
  ;[1 1 1] Widget and interactable trace
  (Utilities|FlowControl|Sequence
    (:then_0
      (Utilities|FlowControl|DoOnce false
        (:Completed
          (bind _returnvalue (Utilities|Time|SetTimerbyEvent (delegate Custom|TraceTick) 0.01 true)))))
    (:then_1
      (Utilities|Time|UnpauseTimerbyHandle _returnvalue))))

(event Custom|StopTraceTick
  ;[1 1 1] Widget and interactable trace
  (Utilities|Time|PauseTimerbyHandle (stale Custom|StartTraceTick _returnvalue)))

(event EventBeginPlay
  (bind _skeletalmesh (Variables|Default|GetSkeletalMesh))
  (Utilities|FlowControl|Sequence
    (:then_0
      (if (Variables|Default|GetisRight)
        ;[1 1 1] Had issues when trying to set first active hand by pawn, because proxy wasn't spawned yet. This solves it
        (CallFunction|MulticastSetHandActive true)
        (else
          (Class|SkinnedMeshComponent|SetSkeletalMesh _skeletalmesh "/Game/OculusHand/HumanHands/l_hand_skeletal.l_hand_skeletal" true)
          (Class|SkeletalMeshComponent|SetAnimClass _skeletalmesh "/Game/OculusHand/HumanHands/BasicHandLeft_AnimBP.BasicHandLeft_AnimBP_C")
          ;[1 1 1] Its necessary to differentiate pointer index from one hand to another. Otherwise widget buttons will flicker while being hovered.
          (Variables|/Script/UMG.WidgetInteractionComponent|SetPointerIndex (Variables|Default|GetWidgetInteraction) 1.0)
          (CallFunction|MulticastSetHandActive false))))
    (:then_1
      (if (not (Variables|Default|GetisShowingLaser))
        (Development|SetHiddeninGame (Variables|Default|GetmeshLaserPath) true false)))
    (:then_2
      (CallFunction|SetAppearance (Variables|Default|Getappearance)))))

(fn ConstructionScript)

(fn Trace
  (params (maxTrace :type Float%20%28single-precision%29))
  (bind _widgetinteraction (Variables|Default|GetWidgetInteraction))
  (bind _returnvalue (Transformation|GetWorldLocation _widgetinteraction))
  (bind (_outhit _returnvalue_2) (Collision|LineTraceByChannel _returnvalue (+ _returnvalue (* (Math|Vector|GetForwardVector _widgetinteraction) maxTrace)) "TraceTypeQuery1" false (Utilities|Array|MakeArray (Components|GetOwner)) "None"))
  (return _outhit _returnvalue_2))

(fn DrawTeleportGizmo
  (params (Array :type Array%20of%20Vectors) (projectedLocation :type Vector) (hasLandedOnValidPlace :type Boolean))
  (bind _returnvalue (select hasLandedOnValidPlace "(R=0.000000,G=0.479320,B=0.119538,A=1.000000)" "(R=0.786000,G=0.052000,B=0.000000,A=1.000000)"))
  (bind _hismteleportpath (Variables|Default|GethismTeleportPath))
  (bind _hismteleportpath_2 (Variables|Default|GethismTeleportPath))
  (bind _returnvalue_2 (Components|InstancedStaticMesh|GetInstanceCount _hismteleportpath))
  (bind _returnvalue_3 (- _returnvalue_2 1))
  (Utilities|FlowControl|Sequence
    (:then_0
      (for _index (range 0 _returnvalue_3)
        (Utilities|Array|Add (LocalVariables|GetinstancesTransforms) (Math|Transform|MakeTransform (.location (CallFunction|GetLocationandTangentInterpolation Array (Math|Float|Fraction (+ (/ (Math|Conversions|ToFloat(Integer) _index) (Math|Conversions|ToFloat(Integer) _returnvalue_3)) (Math|Float|Fraction (* (Utilities|Time|GetRealTimeSeconds) 0.4)))))) (Math|Rotator|MakeRotfromZ (.tangent (CallFunction|GetLocationandTangentInterpolation Array (Math|Float|Fraction (+ (/ (Math|Conversions|ToFloat(Integer) _index) (Math|Conversions|ToFloat(Integer) _returnvalue_3)) (Math|Float|Fraction (* (Utilities|Time|GetRealTimeSeconds) 0.4))))))) "0.050000,0.050000,0.400000")))
      (Class|InstancedStaticMeshComponent|BatchUpdateInstancesTransforms _hismteleportpath_2 0 (LocalVariables|GetinstancesTransforms) true true true)
      (Rendering|Material|SetVectorParameterValueonMaterials _hismteleportpath_2 "color" (Math|Conversions|ToVector(LinearColor) _returnvalue)))
    (:then_1
      (Development|SetHiddeninGame (Variables|Default|GetmeshTeleportTarget) (not hasLandedOnValidPlace) false)
      (if hasLandedOnValidPlace
        (Transformation|SetWorldTransform (Variables|Default|GetmeshTeleportTarget) (Math|Transform|MakeTransform (+ projectedLocation (Variables|Default|GetguardianAreaHostOffset)) "0, 0, 0" "0.500000,2.000000,1") false false)
        (Rendering|Material|SetVectorParameterValueonMaterials (Variables|Default|GetmeshTeleportTarget) "color" (Math|Conversions|ToVector(LinearColor) _returnvalue))))))

(fn ProjectPlayAreatoNavigationSystem
  (params (playAreaCenter :type Vector))
  (bind _guardianareaextent (Variables|Default|GetguardianAreaExtent))
  (bind _guardianareahostoffset (Variables|Default|GetguardianAreaHostOffset))
  (bind _returnvalue (* _guardianareaextent "-1.000000,-1.000000, 0"))
  (bind _returnvalue_2 (* _guardianareaextent "-1.000000,1.000000,0.000000"))
  (bind _returnvalue_3 (* _guardianareaextent "1.000000,1.000000,0.000000"))
  (bind _returnvalue_4 (* _guardianareaextent "1.000000,-1.000000,0.000000"))
  (bind _returnvalue_5 (+ playAreaCenter _returnvalue _guardianareahostoffset))
  (bind _returnvalue_6 (+ playAreaCenter _returnvalue_3 _guardianareahostoffset))
  (bind _returnvalue_7 (+ playAreaCenter _returnvalue_4 _guardianareahostoffset))
  (bind _returnvalue_8 (+ playAreaCenter _returnvalue_2 _guardianareahostoffset))
  (bind (_projectedlocation _returnvalue_9) (AI|Navigation|ProjectPointtoNavigation _returnvalue_8 0 0 "0, 0, 0"))
  (bind (_projectedlocation_2 _returnvalue_10) (AI|Navigation|ProjectPointtoNavigation _returnvalue_5 0 0 "0, 0, 0"))
  (bind (_projectedlocation_3 _returnvalue_11) (AI|Navigation|ProjectPointtoNavigation _returnvalue_6 0 0 "0, 0, 0"))
  (bind (_projectedlocation_4 _returnvalue_12) (AI|Navigation|ProjectPointtoNavigation _returnvalue_7 0 0 "0, 0, 0"))
  (return (- (/ (+ _projectedlocation_3 _projectedlocation_4 _projectedlocation _projectedlocation_2) 4.0) (Variables|Default|GetguardianAreaHostOffset)) (Math|Boolean|ANDBoolean _returnvalue_11 _returnvalue_12 _returnvalue_9 _returnvalue_10)))

(fn SetAppearance
  (params (avatarAppearance :type E_AvatarAppearance%20Enum :default "NewEnumerator0"))
  (bind _output_get (Variables|Default|Setappearance avatarAppearance))
  (Rendering|Material|SetVectorParameterValueonMaterials (Variables|Default|GetSkeletalMesh) "color" (Utilities|Select :Index _output_get :NewEnumerator0 "0.800000,0.800000,0.800000" :NewEnumerator1 "0.000000,0.000000,0.800000" :NewEnumerator2 "0.800000,0.800000,0.000000" :NewEnumerator3 "0.800000,0.000000, 0")))

(fn ScaleMeshBetweenPoints
  (params (meshComp :type Static%20Mesh%20Component%20Object%20Reference) (A :type Vector) (B :type Vector))
  (bind _returnvalue (- B A))
  (Transformation|SetWorldTransform meshComp (Math|Transform|MakeTransform A (Math|Rotator|MakeRotfromX _returnvalue) (Math|Vector|MakeVector (/ (Math|Vector|VectorLength _returnvalue) 1e+02) 0.3 0.3)) false true))

(fn SetLaserColor
  (params (traceHitResult :type E_TraceHitResult%20Enum :default "NewEnumerator0"))
  (Rendering|Material|SetVectorParameterValueonMaterials (Variables|Default|GetmeshLaserPath) "LaserColor" (Math|Conversions|ToVector(LinearColor) (Utilities|Select :Index traceHitResult :NewEnumerator0 "(R=0.718750,G=0.202196,B=0.028606,A=1.000000)" :NewEnumerator1 "(R=0.717647,G=0.200000,B=0.027451,A=1.000000)" :NewEnumerator2 "(R=0.000000,G=0.682292,B=0.209508,A=1.000000)"))))