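; Networked player pawn for VR or PC, with Guide and Visitor avatar looks and server-spawned hands.
; The owning player sends camera and controller transforms to the server on a timer, and non-local copies interpolate toward stored values.
; The host gets a toggleable map menu in UnifiedLevel.
; Teleports move all pawns through the game mode or fall back to a faded solo move; a material sphere handles fades, and timed messages appear as 3D widgets.
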(event Custom|ClientFadeOut
  (params (toColor :type Linear%20Color%20Structure) (duration :type Float%20%28single-precision%29))
  ;[1 1 1] Fade
  (Variables|Default|SetfadeColor toColor)
  (Rendering|SetVisibility (Variables|Default|GetmeshFadeSphere) true false)
  (Components|Timeline|SetPlayRate (Variables|Default|GetTL_FadeMaterial) (/ 1.0 duration))
  (bind (_direction _alpha) (Timeline|TL_FadeMaterial PlayFromStart)
    (:Update
      (Rendering|Material|SetVectorParameterValueonMaterials (Variables|Default|GetmeshFadeSphere) "color" (Math|Conversions|ToVector(LinearColor) (Variables|Default|GetfadeColor)))
      (Rendering|Material|SetScalarParameterValueonMaterials (Variables|Default|GetmeshFadeSphere) "opacity" _alpha))
    (:Finished
      (switch Utilities|FlowControl|Switch|SwitchonETimelineDirection _direction
        (:Forward
          (CallFunction|HideHostMenu))
        (:Backward
          (Rendering|SetVisibility (Variables|Default|GetmeshFadeSphere) false false))))))

(event Custom|ClientFadeIn
  (params (fromColor :type Linear%20Color%20Structure) (duration :type Float%20%28single-precision%29))
  ;[1 1 1] Fade
  (Variables|Default|SetfadeColor fromColor)
  (Utilities|FlowControl|Delay 0.1)
  (Components|Timeline|SetPlayRate (Variables|Default|GetTL_FadeMaterial) (/ 1.0 duration))
  (bind (_direction _alpha) (Timeline|TL_FadeMaterial ReverseFromEnd)
    (:Update
      (Rendering|Material|SetVectorParameterValueonMaterials (Variables|Default|GetmeshFadeSphere) "color" (Math|Conversions|ToVector(LinearColor) (Variables|Default|GetfadeColor)))
      (Rendering|Material|SetScalarParameterValueonMaterials (Variables|Default|GetmeshFadeSphere) "opacity" _alpha))
    (:Finished
      (switch Utilities|FlowControl|Switch|SwitchonETimelineDirection _direction
        (:Forward
          (CallFunction|HideHostMenu))
        (:Backward
          (Rendering|SetVisibility (Variables|Default|GetmeshFadeSphere) false false))))))

(event Custom|SelectHand
  (params (isLeft :type Boolean))
  (Default|MulticastSetHandActive (Variables|Default|GethandLeft) isLeft)
  (Default|MulticastSetHandActive (Variables|Default|GethandRight) (not isLeft)))

(event Custom|VSF
  ;[1 1 1] Interaction on PC
  (CallFunction|ClientFadein :duration 0.23))

(event Custom|ServerSetCameraAndMCsLocationAndRotation
  (params (locations :type Array%20of%20Vectors) (New%20Transform%20Rotation :type Array%20of%20Rotators))
  ;[1 1 1] Camera and motion controllers update from owning player to server
  (Variables|Default|SetCameraAndMCsLocations locations)
  (Variables|Default|SetCameraAndMCsRotations New%20Transform%20Rotation))

(event Custom|SendToServerControlledPawnTransforms
  (bind _camera (Variables|Default|GetCamera))
  (bind _mcleft (Variables|Default|GetmcLeft))
  (bind _mcright (Variables|Default|GetmcRight))
  (bind _returnvalue (Transformation|GetWorldTransform _mcright))
  (bind _returnvalue_2 (Transformation|GetWorldTransform _camera))
  (bind _returnvalue_3 (Transformation|GetWorldTransform _mcleft))
  ;[1 1 1] Camera and motion controllers update from owning player to server
  (CallFunction|ServerSetCameraandMCsLocationandRotation (Utilities|Array|MakeArray (.location _returnvalue_2) (.location _returnvalue_3) (.location _returnvalue)) (Utilities|Array|MakeArray (.rotation _returnvalue_2) (.rotation _returnvalue_3) (.rotation _returnvalue))))

(event Custom|StartTimerToUpdateCameraAndMCsTransforms
  ;[1 1 1] Camera and motion controllers update from owning player to server
  (Utilities|Time|SetTimerbyEvent (delegate Custom|SendToServerControlledPawnTransforms) 0.1 true))

(event Custom|CameraAndMCsInterpolationTick
  ;[1 1 1] Camera and motion controllers update from owning player to server
  (CallFunction|InterpolateCameraandMCsTransforms))

(event Custom|StartInterpolationTickTimer
  ;[1 1 1] Camera and motion controllers update from owning player to server
  (Utilities|Time|SetTimerbyEvent (delegate Custom|CameraAndMCsInterpolationTick) (/ 2.0 72.0) true))

(event Custom|SetFadeAmount
  (params (InFadeAmount :type Float%20%28single-precision%29) (Color :type Linear%20Color%20Structure))
  (bind _meshfadesphere (Variables|Default|GetmeshFadeSphere))
  ;[1 1 1] Fade
  (Variables|Default|SetfadeColor Color)
  (Rendering|Material|SetVectorParameterValueonMaterials _meshfadesphere "color" (Math|Conversions|ToVector(LinearColor) (Variables|Default|GetfadeColor)))
  (Rendering|Material|SetScalarParameterValueonMaterials _meshfadesphere "opacity" InFadeAmount))

(event Custom|ShowHostMenu
  (bind _mapmenu (Variables|Default|GetmapMenu))
  (bind _camera (Variables|Default|GetCamera))
  (bind _returnvalue (Math|Vector|GetForwardVector _camera))
  (bind _returnvalue_2 (* (Math|Vector|MakeVector (.x _returnvalue) (.y _returnvalue) 0.0) 75.0))
  ;[1 1 1] Initializations
  (Utilities|IsValid _mapmenu
    (:Is%20Valid
      (Default|CallOnMapMenuActivated)
      (Transformation|SetActorTransform _mapmenu (Math|Transform|MakeTransform (+ _returnvalue_2 (* (Transformation|GetWorldLocation _camera) "1.000000,1.000000,0.500000")) (Math|Rotator|MakeRotator 0.0 0.0 (.yaw (Math|Rotator|MakeRotfromX _returnvalue_2))) "1,1,1"))
      (Default|SetIsActive _mapmenu true))))

(event Custom|ShowMessageForDuration
  (params (message :type Text) (duration :type Float%20%28single-precision%29))
  (bind _camera (Variables|Default|GetCamera))
  (bind _returnvalue (Transformation|GetWorldLocation _camera))
  (bind _returnvalue_2 (Math|Vector|GetForwardVector _camera))
  (bind _returnvalue_3 (* _returnvalue_2 1e+02))
  (bind _returnvalue_4 (+ _returnvalue _returnvalue_3))
  ;[1 1 1] Message
  (Utilities|FlowControl|DoOnce false :!label _label
    (:Completed
      (bind _returnvalue_5 (Game|SpawnActorfromClass "/Game/SaintGobain/Core/Menus/BP_3DWidget.BP_3DWidget_C" (Math|Transform|MakeTransform _returnvalue_4 (Math|Rotator|FindLookatRotation _returnvalue_4 _returnvalue)) "Undefined" 0 "/Game/SaintGobain/Core/Menus/W_Message.W_Message_C" 1e+02 "(X=400.000000,Y=200.000000)" 0))
      (Actor|SetLifeSpan _returnvalue_5 duration)
      (Transformation|AttachComponentToComponent _returnvalue_5 _camera "None" "KeepWorld" "KeepWorld" "KeepWorld" true)
      (bind _asw_message (Utilities|Casting|CastToW_Message (UserInterface|GetUserWidgetObject (Variables|/Game/SaintGobain/Core/Menus/BP_3DWidget.BP_3DWidget_C|GetWidget _returnvalue_5))))
      (Default|SetText _asw_message message)
      (Utilities|FlowControl|Delay duration)
      (goto _label Reset))))

(event Custom|HideHostMenu
  (bind _mapmenu (Variables|Default|GetmapMenu))
  ;[1 1 1] Initializations
  (Utilities|IsValid _mapmenu
    (:Is%20Valid
      (Default|CallOnMapMenuDeactivated)
      (Default|SetIsActive _mapmenu false))))

(event Custom|SpawnHostMenu
  ;[1 1 1] Initializations
  (bind _returnvalue (Game|SpawnActorfromClass "/Game/SaintGobain/Core/Menus/BP_MapMenu.BP_MapMenu_C" (Math|Transform|MakeTransform (+ (Transformation|GetActorLocation) (Math|Transform|TransformDirection (Transformation|GetActorTransform) "100.000000,0.000000,40.000000")) (Math|Rotator|MakeRotator 0.0 0.0 (.yaw (Transformation|GetActorRotation)))) "Undefined" self 0))
  (bind _output_get (Variables|Default|SetmapMenu _returnvalue))
  (Transformation|AttachActorToActor _output_get self "None" "KeepWorld" "KeepWorld" "KeepWorld" true)
  (CallFunction|HideHostMenu))

(event Custom|StartVRMode
  ;[1 1 1] Initializations
  (Class|HeadMountedDisplayFunctionLibrary|SetTrackingOrigin "Floor")
  (Utilities|FlowControl|Sequence
    (:then_0
      (Utilities|FlowControl|Delay 1.0)
      (bind _returnvalue (Game|GetCurrentLevelName true))
      (if (and (Utilities|Enum|Equal(Enum) _returnvalue "UnifiedLevel") (CallFunction|IsServerOwner))
        (CallFunction|SpawnHostMenu)))
    (:then_1
      (Networking|SwitchHasAuthority
        (:Authority
          (CallFunction|SpawnHands))))))

(event Custom|StartPCMode
  (bind _handright (Variables|Default|GethandRight))
  ;[1 1 1] Initializations
  (Transformation|SetRelativeLocation (Variables|Default|GetCamera) "0, 0,175.000000" false false)
  (Utilities|FlowControl|Sequence
    (:then_0
      (Networking|SwitchHasAuthority
        (:Authority
          (CallFunction|SpawnHands)
          (Transformation|AttachComponentToComponent _handright (Variables|Default|GetCamera) "None" "SnapToTarget" "SnapToTarget" "SnapToTarget" true)
          (Transformation|SetActorRelativeLocation (Variables|Default|GethandLeft) "20.000000,-10.000000,-10.000000")
          (Transformation|SetActorRelativeLocation _handright "20.000000,10.000000,-10.000000"))))
    (:then_1
      (Utilities|FlowControl|Delay 1.0)
      (bind _returnvalue (Game|GetCurrentLevelName true))
      (if (and (Utilities|Enum|Equal(Enum) _returnvalue "UnifiedLevel") (CallFunction|IsServerOwner))
        (CallFunction|SpawnHostMenu)))))

(event Custom|TeleportToLocation
  (params (NewLocation :type Vector))
  (bind _returnvalue (Math|Float|MakeLiteralFloat 0.2))
  ;[1 0.4383 0] Teleport owner only
  (Utilities|FlowControl|DoOnce false :!label _label
    (:Completed
      ;[1 1 1] Teleport all pawns together
      (bind _asbp_sggame_mode (Utilities|Casting|CastToBP_SGGameMode (Game|GetGameMode))
        (:then
          (Default|TeleportActors _asbp_sggame_mode NewLocation true))
        (:CastFailed
          (CallFunction|ClientFadeOut "(R=0.000000,G=0.000000,B=0.000000,A=1.000000)" _returnvalue)
          (Utilities|FlowControl|Delay _returnvalue)
          (Transformation|SetActorLocation NewLocation false true)
          (Class|HeadMountedDisplayFunctionLibrary|ResetOrientationandPosition 0.0 "Position")
          (CallFunction|ClientFadein "(R=0.000000,G=0.000000,B=0.000000,A=1.000000)" _returnvalue)))
      (Utilities|FlowControl|Delay _returnvalue)
      (goto _label Reset))))

(event EventBeginPlay
  ;[1 0.151 0.151] Begin Play
  ;;[1 1 1] Making sure HMD enabled flag is updated
  (Utilities|FlowControl|Delay 0.5)
  (Utilities|FlowControl|Sequence
    (:then_0
      (if (Class|HeadMountedDisplayFunctionLibrary|IsHeadMountedDisplayEnabled)
        (CallFunction|StartVRMode)
        (else
          (CallFunction|StartPCMode))))
    (:then_1
      (if (Pawn|IsLocallyControlled)
        (CallFunction|ClientFadein "(R=0.000000,G=0.000000,B=0.000000,A=1.000000)" 1.0)
        (CallFunction|StartTimertoUpdateCameraandMCsTransforms)
        (else
          (CallFunction|StartInterpolationTickTimer))))
    (:then_2
      ;;[1 1 1] Making collision follow camera position
      (Transformation|DetachFromComponent (Variables|Default|Getcollision) "KeepWorld" "KeepWorld" "KeepWorld" true))
    (:then_3
      (CallFunction|SetAppearance (Variables|Default|GetavatarAppearance)))))

(event EventTick
  (params (DeltaSeconds :type Float%20%28single-precision%29))
  ;[1 0.151 0.151] Begin Play
  ;;[1 1 1] Making collision follow camera position
  (Transformation|SetWorldLocation (Variables|Default|Getcollision) (* (Transformation|GetWorldLocation (Variables|Default|GetCamera)) "1.000000,1.000000,0.500000") false false))

(event Input|ActionEvents|InputActiontriggerRight
  (params (Key :type Key%20Structure :default "None"))
  (bind _returnvalue (Networking|IsServer))
  (bind _handright (Variables|Default|GethandRight))
  ;[1 1 1] Motion controller
  (:Pressed
    (if _returnvalue
      (Default|PressTriggerAction _handright)
      (CallFunction|SelectHand false)))
  (:Released
    (if _returnvalue
      (Default|ReleaseTriggerAction _handright))))

(event Input|ActionEvents|InputActiontriggerLeft
  (params (Key :type Key%20Structure :default "None"))
  (bind _returnvalue (Networking|IsServer))
  (bind _handleft (Variables|Default|GethandLeft))
  ;[1 1 1] Motion controller
  (:Pressed
    (if _returnvalue
      (Default|PressTriggerAction _handleft)
      (CallFunction|SelectHand true)))
  (:Released
    (if _returnvalue
      (Default|ReleaseTriggerAction _handleft))))

(event Input|ActionEvents|InputActiongripLeft
  (params (Key :type Key%20Structure :default "None")))

(event Input|ActionEvents|InputActionfaceButtons
  (params (Key :type Key%20Structure :default "None"))
  ;[1 1 1] Motion controller
  (:Pressed
    (if (and (Networking|IsServer) (Utilities|IsValid (Variables|Default|GetmapMenu)))
      (if (Default|GetIsActive (Variables|Default|GetmapMenu))
        (CallFunction|HideHostMenu)
        (else
          (CallFunction|ShowHostMenu))))))

(event Input|ActionEvents|InputActiongripRight
  (params (Key :type Key%20Structure :default "None")))

(event Input|AxisEvents|InputAxisthumbstickX
  (params (AxisValue :type Float%20%28single-precision%29))
  ;[1 1 1] Motion controller
  ;;[1 1 1] For development only, shouldn't be able to rotate on final version
)

(event Input|MouseEvents|MouseX
  (params (AxisValue :type Float%20%28single-precision%29))
  ;[1 1 1] Interaction on PC
  (if (not (Class|HeadMountedDisplayFunctionLibrary|IsHeadMountedDisplayEnabled))
    (Transformation|AddLocalRotation (Variables|Default|GetVRBase) (Math|Rotator|MakeRotator 0.0 0.0 AxisValue) false false)))

(event Input|MouseEvents|MouseY
  (params (AxisValue :type Float%20%28single-precision%29))
  ;[1 1 1] Interaction on PC
  (if (not (Class|HeadMountedDisplayFunctionLibrary|IsHeadMountedDisplayEnabled))
    (Transformation|SetRelativeRotation (Variables|Default|GetCamera) (Math|Rotator|MakeRotator 0.0 (Math|Float|Clamp(Float) (+ AxisValue (.pitch (Variables|/Script/Engine.SceneComponent|GetRelativeRotation (Variables|Default|GetCamera)))) -89.0 89.0) 0.0) false false)))

(event Input|MouseEvents|LeftMouseButton
  (params (Key :type Key%20Structure :default "None"))
  (bind _handright (Variables|Default|GethandRight))
  ;[1 1 1] Interaction on PC
  (:Pressed
    (Default|PressTriggerAction _handright))
  (:Released
    (Default|ReleaseTriggerAction _handright)))

(event Input|KeyboardEvents|Q
  (params (Key :type Key%20Structure :default "None"))
  ;[1 1 1] Interaction on PC
  (:Pressed
    ;[1 1 1] Motion controller
    (if (and (Networking|IsServer) (Utilities|IsValid (Variables|Default|GetmapMenu)))
      (if (Default|GetIsActive (Variables|Default|GetmapMenu))
        (CallFunction|HideHostMenu)
        (else
          (CallFunction|ShowHostMenu))))))

(event Input|KeyboardEvents|1
  (params (Key :type Key%20Structure :default "None"))
  ;[1 1 1] Interaction on PC
  (:Pressed
    (bind _isa (Utilities|FlowControl|FlipFlop)
      (:A
        _)
      (:B
        _))
    (CallFunction|SelectHand _isa)))

(fn ConstructionScript
  (Rendering|Material|CreateDynamicMaterialInstance (Variables|Default|GetmeshFadeSphere) 0 "/Game/SaintGobain/Art/Player/M_Fade.M_Fade" "None" :!class /Script/Engine.PrimitiveComponent)
  (CallFunction|SetFadeAmount 1.0 "(R=0.000000,G=0.000000,B=0.000000,A=1.000000)"))

(fn SpawnHands
  (Utilities|FlowControl|Sequence
    (:then_0
      (bind _returnvalue (Game|SpawnActorfromClass "/Game/SaintGobain/Core/Player/BP_Hand.BP_Hand_C" (Transformation|GetWorldTransform (Variables|Default|GetVRBase)) "Undefined" self true (CallFunction|IsServerOwner) (Variables|Default|GetavatarAppearance) 0))
      (Transformation|AttachComponentToComponent _returnvalue (Variables|Default|GetmcRight) "None" "SnapToTarget" "SnapToTarget" "KeepWorld" true)
      (Variables|Default|SethandRight _returnvalue))
    (:then_1
      (bind _returnvalue_2 (Game|SpawnActorfromClass "/Game/SaintGobain/Core/Player/BP_Hand.BP_Hand_C" (Transformation|GetWorldTransform (Variables|Default|GetVRBase)) "Undefined" self false (CallFunction|IsServerOwner) (Variables|Default|GetavatarAppearance) 0))
      (Transformation|AttachComponentToComponent _returnvalue_2 (Variables|Default|GetmcLeft) "None" "SnapToTarget" "SnapToTarget" "KeepWorld" true)
      (Variables|Default|SethandLeft _returnvalue_2))))

(fn InterpolateCameraandMCsTransforms
  (bind _returnvalue (Utilities|Time|GetWorldDeltaSeconds))
  (bind _returnvalue_2 (Math|Float|MakeLiteralFloat 15.0))
  (bind _camera (Variables|Default|GetCamera))
  (bind _mcleft (Variables|Default|GetmcLeft))
  (bind _mcright (Variables|Default|GetmcRight))
  (bind _cameraandmcslocations (Variables|Default|GetCameraAndMCsLocations))
  (bind _cameraandmcsrotations (Variables|Default|GetCameraAndMCsRotations))
  (Transformation|SetWorldTransform _camera (Class|KismetMathLibrary|TInterpto (Transformation|GetWorldTransform _camera) (Math|Transform|MakeTransform (Utilities|Array|Get(acopy) _cameraandmcslocations) (Utilities|Array|Get(acopy) _cameraandmcsrotations) "1,1,1") _returnvalue _returnvalue_2) false false)
  (Transformation|SetWorldTransform _mcleft (Class|KismetMathLibrary|TInterpto (Transformation|GetWorldTransform _mcleft) (Math|Transform|MakeTransform (Utilities|Array|Get(acopy) _cameraandmcslocations 1) (Utilities|Array|Get(acopy) _cameraandmcsrotations 1) "1,1,1") _returnvalue _returnvalue_2) false false)
  (Transformation|SetWorldTransform _mcright (Class|KismetMathLibrary|TInterpto (Transformation|GetWorldTransform _mcright) (Math|Transform|MakeTransform (Utilities|Array|Get(acopy) _cameraandmcslocations 2) (Utilities|Array|Get(acopy) _cameraandmcsrotations 2) "1,1,1") _returnvalue _returnvalue_2) false false))

(fn SetAppearance
  (params (avatarAppearance :type E_AvatarAppearance%20Enum :default "NewEnumerator0"))
  (bind _meshhat (Variables|Default|GetmeshHat))
  (bind _output_get (Variables|Default|SetavatarAppearance avatarAppearance))
  (Rendering|Material|SetVectorParameterValueonMaterials (Variables|Default|GetmeshHead) "color" (Utilities|Select :Index _output_get :NewEnumerator0 "0.800000,0.800000,0.800000" :NewEnumerator1 "0.000000,0.000000,0.800000" :NewEnumerator2 "0.800000,0.800000,0.000000" :NewEnumerator3 "0.800000,0.000000, 0"))
  (Development|SetHiddeninGame _meshhat (Utilities|Select :Index _output_get :NewEnumerator0 false :NewEnumerator1 true :NewEnumerator2 true :NewEnumerator3 true) false)
  (Rendering|SetVisibility _meshhat (not (Utilities|Select :Index _output_get :NewEnumerator0 false :NewEnumerator1 true :NewEnumerator2 true :NewEnumerator3 true)) false))

(fn IsServerOwner
  (return (and (Pawn|IsLocallyControlled) (Networking|IsServer))))