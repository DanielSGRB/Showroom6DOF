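; BP_SoundMenu is a menu actor that gathers the level's sound emitter buttons into a row.
; FetchSoundEmittersInLevel orders the first two BP_SoundEmitter actors by Number, assuming at least two exist.
; It attaches each emitter's button to the menu, activates it and spaces it along local Y by index.
; When the menu is destroyed, it deactivates the stored buttons.
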(event EventDestroyed
  (for _array_element (Variables|Default|Getbuttons)
    (Default|SetIsActive _array_element false)))

(fn ConstructionScript)

(fn FetchSoundEmittersinLevel
  (bind _outactors (Actor|GetAllActorsOfClass "/Game/SaintGobain/Core/Interactions/BP_SoundEmitter.BP_SoundEmitter_C"))
  (if (== (Variables|/Game/SaintGobain/Core/Interactions/BP_SoundEmitter.BP_SoundEmitter_C|GetNumber (Utilities|Array|Get(acopy) _outactors)) 1)
    (LocalVariables|SetSoundEmiitersOrder (Utilities|Array|MakeArray (Utilities|Array|Get(acopy) _outactors 1) (Utilities|Array|Get(acopy) _outactors)))
    (else
      (LocalVariables|SetSoundEmiitersOrder (Utilities|Array|MakeArray (Utilities|Array|Get(acopy) _outactors) (Utilities|Array|Get(acopy) _outactors 1)))))
  (for (_array_element _array_index) (LocalVariables|GetSoundEmiitersOrder)
    (Utilities|IsValid _array_element
      (:Is%20Valid
        (Transformation|AttachActorToActor (Default|GetButton _array_element) self "None" "SnapToTarget" "SnapToTarget" "SnapToTarget" false)
        (Utilities|Array|Add (Variables|Default|Getbuttons) (Default|GetButton _array_element))
        (Default|SetIsActive (Default|GetButton _array_element) true)
        (Transformation|SetActorRelativeLocation (Default|GetButton _array_element) (Math|Vector|MakeVector 0.0 (* (- (Math|Conversions|ToFloat(Integer) _array_index) (/ (Math|Conversions|ToFloat(Integer) (Utilities|Array|Length (LocalVariables|GetSoundEmiitersOrder))) 2.0)) 3e+01) 0.0))))))