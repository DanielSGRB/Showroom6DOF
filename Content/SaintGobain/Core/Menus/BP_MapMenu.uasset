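; Map menu actor that presents selectable map buttons in an arc around itself and toggles them along with a sound menu.
; On BeginPlay it rebuilds attached BP_MapButton actors: five large map buttons plus two smaller non-map buttons on a nearer arc, all facing the center.
; SetIsActive propagates state to the buttons and spawns BP_SoundMenu, populated with level sound emitters, or destroys it.
; The construction script draws debug points to preview button placement.
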(event EventBeginPlay
  (CallFunction|ClearOldandSpawnNewButtons))

(fn ConstructionScript
  (for _index (range 0 5)
    (Rendering|Debug|DrawDebugPoint (.location (CallFunction|GetButtonTransformbyIndex _index 5e+01 2e+01)) 0.0 "(R=1.000000,G=0.000000,B=0.000000,A=1.000000)" 1e+01)))

(fn GetButtonTransformbyIndex
  (params (index :type Integer) (distanceFromOrigin :type Float%20%28single-precision%29) (spacingAngle :type Float%20%28single-precision%29) (lastIndex :type Integer))
  (bind _returnvalue (Transformation|GetActorForwardVector))
  (bind _returnvalue_2 (Transformation|GetActorLocation))
  (bind _returnvalue_3 (Math|Conversions|ToFloat(Integer) index))
  (bind _returnvalue_4 (Math|Conversions|ToFloat(Integer) lastIndex))
  (bind _returnvalue_5 (/ _returnvalue_4 2.0))
  (bind _returnvalue_6 (- _returnvalue_3 _returnvalue_5))
  (bind _returnvalue_7 (* _returnvalue_6 spacingAngle))
  (bind _returnvalue_8 (Math|Vector|RotateVectorAroundAxis _returnvalue _returnvalue_7 "0, 0,1.000000"))
  (bind _returnvalue_9 (* _returnvalue_8 distanceFromOrigin))
  (bind _returnvalue_10 (+ _returnvalue_9 _returnvalue_2))
  (return (Math|Transform|MakeTransform _returnvalue_10 (Math|Rotator|FindLookatRotation _returnvalue_10 _returnvalue_2) "1,1,1")))

(fn ClearOldandSpawnNewButtons
  (Utilities|FlowControl|Sequence
    (:then_0
      (for _array_element (Variables|Default|Getbuttons)
        (Actor|DestroyActor _array_element))
      (Utilities|Array|Clear (Variables|Default|Getbuttons)))
    (:then_1
      (for (_array_element_2 _array_index) (Utilities|Array|MakeArray "NewEnumerator4" "NewEnumerator0" "NewEnumerator1" "NewEnumerator3" "NewEnumerator2" "NewEnumerator5" "NewEnumerator5")
        (bind _returnvalue (Game|SpawnActorfromClass "/Game/SaintGobain/Core/Interactions/BP_MapButton.BP_MapButton_C" (select (Utilities|Enum|Equal(Enum) _array_element_2 "NewEnumerator5") (CallFunction|GetButtonTransformbyIndex (- _array_index 5) 5e+01 2e+01 1) (CallFunction|GetButtonTransformbyIndex _array_index 1e+02 2e+01 4)) "Undefined" 0 _array_element_2 (select (Utilities|Enum|Equal(Enum) _array_element_2 "NewEnumerator5") 15.0 35.0) (select (Utilities|Enum|Equal(Enum) _array_element_2 "NewEnumerator5") (- _array_index 5) 2) 0))
        (Utilities|Array|Add (Variables|Default|Getbuttons) _returnvalue)
        (Transformation|AttachActorToActor _returnvalue self "None" "KeepWorld" "KeepWorld" "KeepWorld" true)))))

(fn SetIsActive
  (params (isActive :type Boolean))
  (bind _returnvalue (Transformation|GetActorTransform))
  (Variables|Default|SetisActive isActive)
  (for _array_element (Variables|Default|Getbuttons)
    (Default|SetIsActive _array_element isActive))
  (if isActive
    (bind _returnvalue_2 (Game|SpawnActorfromClass "/Game/SaintGobain/Core/Menus/BP_SoundMenu.BP_SoundMenu_C" (Math|Transform|MakeTransform (+ (.location _returnvalue) "0, 0,50.000000" (* (Math|Vector|GetForwardVector (.rotation _returnvalue)) 1e+02)) (Math|Rotator|CombineRotators (.rotation _returnvalue) "0,180.000000, 0") "1,1,1") "Undefined" 0 0))
    (bind _output_get (Variables|Default|SetsoundMenu _returnvalue_2))
    (Default|FetchSoundEmittersinLevel _output_get)
    (else
      (Utilities|IsValid (Variables|Default|GetsoundMenu)
        (:Is%20Valid
          (Actor|DestroyActor (Variables|Default|GetsoundMenu)))
        (:Is%20Not%20Valid
          _))
      (Variables|Default|SetsoundMenu 0))))

(fn GetIsActive
  (return (Variables|Default|GetisActive)))