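; BP_ConfirmationMenu is a world-space yes/no confirmation prompt actor with Portuguese button labels.
; On BeginPlay it spawns two BP_Button actors either side of itself, sized by SpheresSize, and rebroadcasts their presses through OnConfirmationResult as true or false.
; The construction script scales and raises the prompt text from SpheresSize.
; It destroys both buttons when it is destroyed.
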(event Custom|Negate
  (params (buttonRef :type BP%20Button%20Object%20Reference))
  (Default|CallOnConfirmationResult false))

(event Custom|Confirm
  (params (buttonRef :type BP%20Button%20Object%20Reference))
  (Default|CallOnConfirmationResult true))

(event EventBeginPlay
  (bind _spheressize (Variables|Default|GetspheresSize))
  (Utilities|FlowControl|Sequence
    (:then_0
      (bind _returnvalue (Game|SpawnActorfromClass "/Game/SaintGobain/Core/Interactions/BP_Button.BP_Button_C" (Math|Transform|ComposeTransforms (Math|Transform|MakeTransform "0,20.000000, 0") (Transformation|GetActorTransform)) "Undefined" 0 _spheressize "Sim" false 0))
      (Utilities|Array|Add (Variables|Default|Getbuttons) _returnvalue)
      (EventDispatchers|BindEventtoOnButtonPressed _returnvalue (delegate Custom|Confirm)))
    (:then_1
      (bind _returnvalue_2 (Game|SpawnActorfromClass "/Game/SaintGobain/Core/Interactions/BP_Button.BP_Button_C" (Math|Transform|ComposeTransforms (Math|Transform|MakeTransform "0,-20.000000, 0") (Transformation|GetActorTransform)) "Undefined" 0 _spheressize "Não" false 0))
      (Utilities|Array|Add (Variables|Default|Getbuttons) _returnvalue_2)
      (EventDispatchers|BindEventtoOnButtonPressed _returnvalue_2 (delegate Custom|Negate)))))

(event EventDestroyed
  (for _array_element (Variables|Default|Getbuttons)
    (Actor|DestroyActor _array_element)))

(fn ConstructionScript
  (Rendering|Components|TextRender|SetWorldSize (Variables|Default|GetTextRender) (/ (Math|Float|Max(Float) (Variables|Default|GetspheresSize) 35.0) 5.0))
  (Transformation|SetRelativeLocation (Variables|Default|GetTextRender) (Math|Vector|MakeVector 0.0 0.0 (Variables|Default|GetspheresSize)) false false))