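; BP_3DWidget is a reusable Blueprint that displays a configurable user widget in the 3D world through its widget component.
; The construction script sets the draw size and scales the component uniformly in Y and Z, so WidgetWidth defines world width independently of pixel resolution.
; On BeginPlay it constructs an instance of WidgetClass with the component as outer and assigns it if it casts to UserWidget.
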(event EventBeginPlay
  (bind _widget (Variables|Default|GetWidget))
  (bind _returnvalue (Game|ConstructObjectfromClass (Variables|Default|GetwidgetClass) _widget))
  (bind _asuser_widget (Utilities|Casting|CastToUserWidget _returnvalue))
  (UserInterface|SetWidget _widget _asuser_widget))

(fn ConstructionScript
  (bind _widgetwidth (Variables|Default|GetwidgetWidth))
  (bind _drawsize (Variables|Default|GetdrawSize))
  (bind _returnvalue (/ _widgetwidth (.x _drawsize)))
  (Transformation|SetWorldScale3D (Variables|Default|GetWidget) (Math|Vector|MakeVector 1.0 _returnvalue _returnvalue))
  (Class|WidgetComponent|SetDrawSize (Variables|Default|GetWidget) (Variables|Default|GetdrawSize)))